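; Gameplay ability that cycles the combat character to the next ranged weapon, wrapping at the array's end and guarded by an IsSwitchingWeapon flag.
; It clears the active weapon's primary/secondary abilities and reattaches it to its inventory socket.
; The next weapon links its anim layer, plays an equip montage and grants abilities on the Event.Equip.PhotonRifle event.
; It attaches to hand_r; the server calls MCSelectWeapon, then ends the ability after a delay.
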(event Custom|SwitchWeaponSetFalse)

(event Ability|EventActivateAbility
  ;[1 1 1] ActivateAbility Store Combat CharacterRef
  (bind _asbp_combat_character (Utilities|Casting|CastToBP_CombatCharacter (Ability|GetAvatarActorfromActorInfo))
    (:then
      (bind _output_get (Variables|Default|SetAs%20BP%20Combat%20Character _asbp_combat_character))
      ;[1 1 1] Check if Character is Currently Switching Weapons(EndAbility if currently Switching)
      (if (Variables|/Game/Blueprints/Character/BP_CombatCharacter.BP_CombatCharacter_C|GetIsSwitchingWeapon? _output_get)
        (Ability|EndAbility)
        (else
          (Variables|/Game/Blueprints/Character/BP_CombatCharacter.BP_CombatCharacter_C|SetIsSwitchingWeapon? _output_get true)
          (Ability|CommitAbility)
          ;[1 1 1] Put Active weapon Back into inventory slot
          (CallFunction|PutWeaponBacktoInventory)
          ;[1 1 1 1 42] Check if WeaponInventory Array Length and Current Weapon Index are same(if not the same, increment Active Index and Get Corresponding Weapon from Array and Equip to Hand
          (if (== (Variables|/Script/CombatGASCompanion.CombatCharacter|GetActiveWeaponIndex (Variables|Default|GetAs%20BP%20Combat%20Character)) (- (Utilities|Array|Length (Variables|/Script/CombatGASCompanion.CombatCharacter|GetCombatRangedWeaponsArray (Variables|Default|GetAs%20BP%20Combat%20Character))) 1))
            (Utilities|PlayWeaponEquipMontage (Utilities|Array|Get(acopy) (Variables|/Script/CombatGASCompanion.CombatCharacter|GetCombatRangedWeaponsArray (Variables|Default|GetAs%20BP%20Combat%20Character))))
            (Utilities|IsValid (Utilities|Array|Get(acopy) (Variables|/Script/CombatGASCompanion.CombatCharacter|GetCombatRangedWeaponsArray (Variables|Default|GetAs%20BP%20Combat%20Character)))
              (:Is%20Valid
                (Transformation|AttachComponentToComponent (Utilities|Array|Get(acopy) (Variables|/Script/CombatGASCompanion.CombatCharacter|GetCombatRangedWeaponsArray (Variables|Default|GetAs%20BP%20Combat%20Character))) (Variables|/Script/Engine.Character|GetMesh (Variables|Default|GetAs%20BP%20Combat%20Character)) "hand_r" "SnapToTarget" "SnapToTarget" "SnapToTarget" true)
                (if (Networking|IsServer)
                  (Default|MCSelectWeapon (Variables|Default|GetAs%20BP%20Combat%20Character) 0 (Variables|/Script/CombatGASCompanion.CombatRangedWeapon|GetWeaponPropertiesStructure (Utilities|Array|Get(acopy) (Variables|/Script/CombatGASCompanion.CombatCharacter|GetCombatRangedWeaponsArray (Variables|Default|GetAs%20BP%20Combat%20Character)))))
                  (Ability|Tasks|WaitDelay 2.0 :!label _label
                    (:OnFinish
                      (Variables|/Game/Blueprints/Character/BP_CombatCharacter.BP_CombatCharacter_C|SetIsSwitchingWeapon? (Variables|Default|GetAs%20BP%20Combat%20Character) false)
                      (Ability|EndAbility))))))
            (else
              (Utilities|PlayWeaponEquipMontage (Utilities|Array|Get(acopy) (Variables|/Script/CombatGASCompanion.CombatCharacter|GetCombatRangedWeaponsArray (Variables|Default|GetAs%20BP%20Combat%20Character)) (+ (Variables|/Script/CombatGASCompanion.CombatCharacter|GetActiveWeaponIndex (Variables|Default|GetAs%20BP%20Combat%20Character)) 1)))
              (Utilities|IsValid (Utilities|Array|Get(acopy) (Variables|/Script/CombatGASCompanion.CombatCharacter|GetCombatRangedWeaponsArray (Variables|Default|GetAs%20BP%20Combat%20Character)) (+ (Variables|/Script/CombatGASCompanion.CombatCharacter|GetActiveWeaponIndex (Variables|Default|GetAs%20BP%20Combat%20Character)) 1))
                (:Is%20Valid
                  (Transformation|AttachComponentToComponent (Utilities|Array|Get(acopy) (Variables|/Script/CombatGASCompanion.CombatCharacter|GetCombatRangedWeaponsArray (Variables|Default|GetAs%20BP%20Combat%20Character)) (+ (Variables|/Script/CombatGASCompanion.CombatCharacter|GetActiveWeaponIndex (Variables|Default|GetAs%20BP%20Combat%20Character)) 1)) (Variables|/Script/Engine.Character|GetMesh (Variables|Default|GetAs%20BP%20Combat%20Character)) "hand_r" "SnapToTarget" "SnapToTarget" "SnapToTarget" true)
                  (if (Networking|IsServer)
                    (Default|MCSelectWeapon (Variables|Default|GetAs%20BP%20Combat%20Character) (+ (Variables|/Script/CombatGASCompanion.CombatCharacter|GetActiveWeaponIndex (Variables|Default|GetAs%20BP%20Combat%20Character)) 1) (Variables|/Script/CombatGASCompanion.CombatRangedWeapon|GetWeaponPropertiesStructure (Utilities|Array|Get(acopy) (Variables|/Script/CombatGASCompanion.CombatCharacter|GetCombatRangedWeaponsArray (Variables|Default|GetAs%20BP%20Combat%20Character)) (+ (Variables|/Script/CombatGASCompanion.CombatCharacter|GetActiveWeaponIndex (Variables|Default|GetAs%20BP%20Combat%20Character)) 1))))
                    (goto _label)))))))))
    (:CastFailed
      (Ability|EndAbility))))

(event Ability|EventOnEndAbility
  (params (bWasCancelled :type Boolean)))

(fn PutWeaponBacktoInventory
  (bind _returnvalue (Ability|GetAbilitySystemComponentfromActorInfo))
  (bind _returnvalue_2 (Ability|GetAbilitySystemComponentfromActorInfo))
  (bind _as_bp_combat_character (Variables|Default|GetAs%20BP%20Combat%20Character))
  (bind _as_bp_combat_character_2 (Variables|Default|GetAs%20BP%20Combat%20Character))
  (bind _activeweaponindex (Variables|/Script/CombatGASCompanion.CombatCharacter|GetActiveWeaponIndex _as_bp_combat_character_2))
  (bind _combatrangedweaponsarray (Variables|/Script/CombatGASCompanion.CombatCharacter|GetCombatRangedWeaponsArray _as_bp_combat_character_2))
  (bind _output (Utilities|Array|Get(acopy) _combatrangedweaponsarray _activeweaponindex))
  (bind _weaponpropertiesstructure (Variables|/Script/CombatGASCompanion.CombatRangedWeapon|GetWeaponPropertiesStructure _output))
  (bind (_displayname _bisautofire _bisshotgun _firerate _ammo_clip _ammo_stock _weaponprimary _weaponsecondary _firemontage _equipmontage _reloadmontage _weaponfiremontage _inventoryslot) (Utilities|Struct|BreakWeaponProperties _weaponpropertiesstructure))
  (Utilities|IsValid (Utilities|Array|Get(acopy) (Variables|/Script/CombatGASCompanion.CombatCharacter|GetCombatRangedWeaponsArray _as_bp_combat_character) (Variables|/Script/CombatGASCompanion.CombatCharacter|GetActiveWeaponIndex _as_bp_combat_character))
    (:Is%20Valid
      (bind _outabilityhandles (Class|AbilitySystemComponent|GetAllAbilities _returnvalue_2))
      (for _array_element _outabilityhandles
        (if (== (Utilities|GetClass (.ReturnValue (Ability|GameplayAbility|GetGameplayAbilityfromSpecHandle _returnvalue_2 _array_element))) _weaponprimary)
          (GameplayAbilities|ClearAbility _returnvalue _array_element)
          (elif (== (Utilities|GetClass (.ReturnValue (Ability|GameplayAbility|GetGameplayAbilityfromSpecHandle _returnvalue_2 _array_element))) _weaponsecondary)
            (GameplayAbilities|ClearAbility _returnvalue _array_element)
            (else
              (Development|PrintString "NO ABILITIES TO CLEAR")))))
      (Utilities|IsValid _output
        (:Is%20Valid
          (Transformation|AttachComponentToComponent _output (Variables|/Script/Engine.Character|GetMesh _as_bp_combat_character_2) _inventoryslot "SnapToTarget" "SnapToTarget" "KeepRelative" true))
        (:Is%20Not%20Valid
          _)))
    (:Is%20Not%20Valid
      _))
  (return))