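; GA_Death is a gameplay ability that plays the death sequence for a Test_EnemyPawn.
; On activation it applies GE_Death, stops pawn movement and plays WalkerRobot_Death_Montage while disabling collision on the skeletal mesh.
; Animations pause at montage blend-out to hold the final pose.
; When the montage completes, is interrupted or is cancelled, it removes the effect and ends the ability.
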(event Ability|EventActivateAbility
  (bind _returnvalue (Ability|ApplyGameplayEffectToOwner "/Game/Blueprints/AbilitySystem/GameplayEffects/GE_Death.GE_Death_C"))
  (Variables|Default|SetActive%20GEHandle _returnvalue)
  (bind _astest_enemy_pawn (Utilities|Casting|CastToTest_EnemyPawn (Ability|GetAvatarActorfromActorInfo)))
  (Class|NavMovementComponent|StopActiveMovement (Variables|/Script/CombatGASCompanion.MinionCharacter|GetPawnMovement _astest_enemy_pawn))
  (|PlayMontageandWaitProxy "None" "/Game/ImportedContent/WalkerRobot_Death_Montage.WalkerRobot_Death_Montage" 1.0 "None" true 1.0 0.0
    (:then
      (Collision|SetCollisionEnabled (Variables|/Script/CombatGASCompanion.EnemyPawnBase|GetSkeletalMeshComponent _astest_enemy_pawn) "NoCollision"))
    (:OnCompleted
      (Ability|RemoveGameplayEffectFromOwnerWithHandle (Variables|Default|GetActive%20GEHandle) :!label _label)
      (Ability|EndAbility))
    (:OnBlendOut
      (Variables|/Script/Engine.SkeletalMeshComponent|SetbPauseAnims (Variables|/Script/CombatGASCompanion.EnemyPawnBase|GetSkeletalMeshComponent _astest_enemy_pawn) true))
    (:OnInterrupted
      (goto _label))
    (:OnCancelled
      (goto _label))))

(event Ability|EventOnEndAbility
  (params (bWasCancelled :type Boolean)))