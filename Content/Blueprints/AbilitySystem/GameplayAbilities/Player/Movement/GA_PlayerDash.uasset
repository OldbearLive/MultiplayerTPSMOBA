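; Player dash gameplay ability that boosts jet movement for a set duration, with gameplay cues for start and stop.
; Activation outside jet mode dashes immediately and triggers the Jet ability; when already jetting, it waits for an input press.
; Each dash toggles the movement component's Dash flag and server dashing state, then re-arms after a short delay.
; While armed, it listens for JetStop events and a movement-component end-jet callback to end the ability.
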(event Custom|ResetDashPressed
  (Ability|Tasks|WaitDelay 0.1
    (:OnFinish
      (Ability|Tasks|WaitInputPress false
        (:then
          (bind _asynctaskproxy (Ability|Tasks|WaitGameplayEvent "(TagName=\"Event.Movement.JetStop\")" 0 true)
            (:then
              (Variables|Default|SetWaitEventTask _asynctaskproxy)
              (EventDispatchers|BindEventtoEndJet (Variables|Default|GetCombat%20Character%20Movement%20Component) (EventDispatchers|CreateEvent :!event Custom|ON%20EndJet)))
            (:EventReceived
              (Ability|EndAbility))))
        (:OnPress
          (Variables|/Script/CombatGASCompanion.CombatCharacterMovementComponent|SetbDash (Variables|Default|GetCombat%20Character%20Movement%20Component) true)
          (Class|CombatCharacter|ServerSetDashing (Variables|Default|GetAs%20BP%20Combat%20Character) true)
          (Class|GameplayAbility|ExecuteGameplayCuewithParams "(TagName=\"GameplayCue.Movement.Jet.Dash\")" (Ability|GameplayCue|MakeGameplayCueParameters :Instigator (Variables|Default|GetAs%20BP%20Combat%20Character)))
          (Ability|Tasks|WaitDelay (Variables|Default|GetDashDuration)
            (:OnFinish
              (Variables|/Script/CombatGASCompanion.CombatCharacterMovementComponent|SetbDash (Variables|Default|GetCombat%20Character%20Movement%20Component) false)
              (Class|CombatCharacter|ServerSetDashing (Variables|Default|GetAs%20BP%20Combat%20Character) false)
              (Class|GameplayAbility|ExecuteGameplayCuewithParams "(TagName=\"GameplayCue.Movement.Jet.DashStop\")" (Ability|GameplayCue|MakeGameplayCueParameters :Instigator (Variables|Default|GetAs%20BP%20Combat%20Character)))
              (bind _waiteventtask (Variables|Default|GetWaitEventTask)
                (:then
                  (GameplayTasks|EndTask _waiteventtask))
                (:else
                  _))
              (CallFunction|ResetDashPressed))))))))

(event Custom|ON%20EndJet
  (Variables|/Script/CombatGASCompanion.CombatCharacterMovementComponent|SetbDash (Variables|Default|GetCombat%20Character%20Movement%20Component) false)
  (Class|CombatCharacter|ServerSetDashing (Variables|Default|GetAs%20BP%20Combat%20Character) false)
  (Class|GameplayAbility|ExecuteGameplayCuewithParams "(TagName=\"GameplayCue.Movement.Jet.DashStop\")" (Ability|GameplayCue|MakeGameplayCueParameters :Instigator (Variables|Default|GetAs%20BP%20Combat%20Character)))
  (Ability|EndAbility))

(event Ability|EventActivateAbility
  (bind _asbp_combat_character (Utilities|Casting|CastToBP_CombatCharacter (Ability|GetAvatarActorfromActorInfo)))
  (Variables|Default|SetAs%20BP%20Combat%20Character _asbp_combat_character)
  (bind _output_get (Variables|Default|SetCombat%20Character%20Movement%20Component (Variables|/Script/CombatGASCompanion.CombatCharacter|GetCombatCharacterMovementComponent _asbp_combat_character)))
  (Variables|Default|SetDefaultFriction (Variables|/Script/CombatGASCompanion.CombatCharacterMovementComponent|GetJetPack_Friction _output_get))
  (Ability|CommitAbility)
  (bind _returnvalue (Class|CombatCharacterMovementComponent|IsCustomMovementMode (Variables|Default|GetCombat%20Character%20Movement%20Component) "CMOVE_JET"))
  (if (or _returnvalue (GameplayTags|HasMatchingGameplayTag (Ability|GetAbilitySystemComponentfromActorInfo) "(TagName=\"Effects.Movement.Jet\")"))
    (Ability|Tasks|WaitInputPress false
      (:then
        (bind _asynctaskproxy (Ability|Tasks|WaitGameplayEvent "(TagName=\"Event.Movement.JetStop\")" 0 true)
          (:then
            (Variables|Default|SetWaitEventTask _asynctaskproxy)
            (EventDispatchers|BindEventtoEndJet (Variables|Default|GetCombat%20Character%20Movement%20Component) (EventDispatchers|CreateEvent :!event Custom|ON%20EndJet)))
          (:EventReceived
            (Ability|EndAbility))))
      (:OnPress
        (Variables|/Script/CombatGASCompanion.CombatCharacterMovementComponent|SetbDash (Variables|Default|GetCombat%20Character%20Movement%20Component) true)
        (Class|CombatCharacter|ServerSetDashing (Variables|Default|GetAs%20BP%20Combat%20Character) true)
        (Class|GameplayAbility|ExecuteGameplayCuewithParams "(TagName=\"GameplayCue.Movement.Jet.Dash\")" (Ability|GameplayCue|MakeGameplayCueParameters :Instigator (Variables|Default|GetAs%20BP%20Combat%20Character)))
        (Ability|Tasks|WaitDelay (Variables|Default|GetDashDuration)
          (:OnFinish
            (Variables|/Script/CombatGASCompanion.CombatCharacterMovementComponent|SetbDash (Variables|Default|GetCombat%20Character%20Movement%20Component) false)
            (Class|CombatCharacter|ServerSetDashing (Variables|Default|GetAs%20BP%20Combat%20Character) false)
            (Class|GameplayAbility|ExecuteGameplayCuewithParams "(TagName=\"GameplayCue.Movement.Jet.DashStop\")" (Ability|GameplayCue|MakeGameplayCueParameters :Instigator (Variables|Default|GetAs%20BP%20Combat%20Character)))
            (bind _waiteventtask (Variables|Default|GetWaitEventTask)
              (:then
                (GameplayTasks|EndTask _waiteventtask))
              (:else
                _))
            (CallFunction|ResetDashPressed)))))
    (else
      (Variables|/Script/CombatGASCompanion.CombatCharacterMovementComponent|SetbDash (Variables|Default|GetCombat%20Character%20Movement%20Component) true)
      (Class|CombatCharacter|ServerSetDashing (Variables|Default|GetAs%20BP%20Combat%20Character) true)
      (Abilities|TryActivateAbilitiesbyTag (Ability|GetAbilitySystemComponentfromActorInfo) (GameplayTags|MakeLiteralGameplayTagContainer "(GameplayTags=((TagName=\"Abilities.Movement.Jet\")))") true)
      (Class|GameplayAbility|ExecuteGameplayCuewithParams "(TagName=\"GameplayCue.Movement.Jet.Dash\")" (Ability|GameplayCue|MakeGameplayCueParameters :Instigator (Variables|Default|GetAs%20BP%20Combat%20Character)))
      (Ability|Tasks|WaitDelay (Variables|Default|GetDashDuration)
        (:OnFinish
          (Variables|/Script/CombatGASCompanion.CombatCharacterMovementComponent|SetbDash (Variables|Default|GetCombat%20Character%20Movement%20Component) false)
          (Class|CombatCharacter|ServerSetDashing (Variables|Default|GetAs%20BP%20Combat%20Character) false)
          (Class|GameplayAbility|ExecuteGameplayCuewithParams "(TagName=\"GameplayCue.Movement.Jet.DashStop\")" (Ability|GameplayCue|MakeGameplayCueParameters :Instigator (Variables|Default|GetAs%20BP%20Combat%20Character)))
          (bind _waiteventtask_2 (Variables|Default|GetWaitEventTask)
            (:then
              (GameplayTasks|EndTask _waiteventtask_2))
            (:else
              _))
          (CallFunction|ResetDashPressed))))))

(event Ability|EventOnEndAbility
  (params (bWasCancelled :type Boolean))
  (Variables|/Script/CombatGASCompanion.CombatCharacterMovementComponent|SetbDash (Variables|Default|GetCombat%20Character%20Movement%20Component) false)
  (Class|CombatCharacter|ServerSetDashing (Variables|Default|GetAs%20BP%20Combat%20Character) false)
  (Class|GameplayAbility|ExecuteGameplayCuewithParams "(TagName=\"GameplayCue.Movement.Jet.DashStop\")" (Ability|GameplayCue|MakeGameplayCueParameters :Instigator (Variables|Default|GetAs%20BP%20Combat%20Character))))