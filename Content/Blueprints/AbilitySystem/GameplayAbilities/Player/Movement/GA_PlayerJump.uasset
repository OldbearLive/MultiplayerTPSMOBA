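; Player jump gameplay ability that calls Jump on the owning combat character and ends immediately.
; It also holds jetpack hover logic that the activation path never reaches.
; That dormant logic uses timed input press and release tasks to enter via montage, toggle thrust on the movement component, link or unlink the jetpack anim layer and restore gravity on exit.
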(event Custom|HoverStateSet
  (bind _timewaited (Ability|Tasks|WaitInputPress false)
    (:OnPress
      (if (> _timewaited 0.5)
        (Ability|Tasks|WaitInputRelease false
          (:then
            (Variables|/Script/CombatGASCompanion.CombatCharacterMovementComponent|SetbThrust (Variables|Default|GetCombat%20Character%20Movement%20Component) true))
          (:OnRelease
            (Variables|/Script/CombatGASCompanion.CombatCharacterMovementComponent|SetbThrust (Variables|Default|GetCombat%20Character%20Movement%20Component) false)
            (CallFunction|HoverStateSet)))
        (else
          (Class|CombatCharacterMovementComponent|JetReleased (Variables|Default|GetCombat%20Character%20Movement%20Component))
          (Default|MCUnlinkAnimLayer (Variables|Default|GetAs%20BP%20Combat%20Character) "/Game/Blueprints/Character/Animation/ABP_Jetpack.ABP_Jetpack_C")
          (Variables|/Script/Engine.CharacterMovementComponent|SetGravityScale (Variables|Default|GetCombat%20Character%20Movement%20Component) 1.0)
          (Ability|EndAbility))))))

(event Ability|EventActivateAbility
  (bind _asbp_combat_character (Utilities|Casting|CastToBP_CombatCharacter (Ability|GetAvatarActorfromActorInfo)))
  (Variables|Default|SetAs%20BP%20Combat%20Character _asbp_combat_character)
  (Variables|Default|SetCombat%20Character%20Movement%20Component (Variables|/Script/CombatGASCompanion.CombatCharacter|GetCombatCharacterMovementComponent _asbp_combat_character))
  (Character|Jump (Variables|Default|GetAs%20BP%20Combat%20Character))
  (Ability|EndAbility))

(event Ability|EventOnEndAbility
  (params (bWasCancelled :type Boolean)))