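; Player jet thrust gameplay ability that toggles the Thrust flag on the combat character's movement component with ability input.
; It runs only in custom JET movement mode or with the Effects.Movement.Jet tag, otherwise ending immediately.
; Input press sets Thrust; release clears it and re-arms the wait tasks in a loop.
; A JetStop gameplay event ends the ability, and OnEndAbility clears Thrust.
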(event Custom|Reset%20Wait%20InputPress
  (Ability|Tasks|WaitInputPress false
    (:then
      (bind _asynctaskproxy (Ability|Tasks|WaitGameplayEvent "(TagName=\"Event.Movement.JetStop\")" 0 true)
        (:then
          (bind _asynctaskproxy_2 (Ability|Tasks|WaitInputRelease false)
            (:OnRelease
              (GameplayTasks|EndTask _asynctaskproxy)
              (GameplayTasks|EndTask _asynctaskproxy_2)
              (Variables|/Script/CombatGASCompanion.CombatCharacterMovementComponent|SetbThrust (Variables|Default|GetCombat%20Character%20Movement%20Component) false)
              (CallFunction|ResetWaitInputPress))))
        (:EventReceived
          (Ability|EndAbility))))
    (:OnPress
      (Variables|/Script/CombatGASCompanion.CombatCharacterMovementComponent|SetbThrust (Variables|Default|GetCombat%20Character%20Movement%20Component) true))))

(event Ability|EventActivateAbility
  (Ability|CommitAbility)
  (bind _asbp_combat_character (Utilities|Casting|CastToBP_CombatCharacter (Ability|GetAvatarActorfromActorInfo)))
  (Variables|Default|SetAs%20BP%20Combat%20Character _asbp_combat_character)
  (bind _output_get (Variables|Default|SetCombat%20Character%20Movement%20Component (Variables|/Script/CombatGASCompanion.CombatCharacter|GetCombatCharacterMovementComponent _asbp_combat_character)))
  (bind _returnvalue (Class|CombatCharacterMovementComponent|IsCustomMovementMode _output_get "CMOVE_JET"))
  (if (or _returnvalue (GameplayTags|HasMatchingGameplayTag (Ability|GetAbilitySystemComponentfromActorInfo) "(TagName=\"Effects.Movement.Jet\")"))
    (Ability|Tasks|WaitInputPress false
      (:then
        (bind _asynctaskproxy (Ability|Tasks|WaitGameplayEvent "(TagName=\"Event.Movement.JetStop\")" 0 true)
          (:then
            (bind _asynctaskproxy_2 (Ability|Tasks|WaitInputRelease false)
              (:OnRelease
                (GameplayTasks|EndTask _asynctaskproxy)
                (GameplayTasks|EndTask _asynctaskproxy_2)
                (Variables|/Script/CombatGASCompanion.CombatCharacterMovementComponent|SetbThrust (Variables|Default|GetCombat%20Character%20Movement%20Component) false)
                (CallFunction|ResetWaitInputPress))))
          (:EventReceived
            (Ability|EndAbility))))
      (:OnPress
        (Variables|/Script/CombatGASCompanion.CombatCharacterMovementComponent|SetbThrust (Variables|Default|GetCombat%20Character%20Movement%20Component) true)))
    (else
      (Ability|EndAbility))))

(event Ability|EventOnEndAbility
  (params (bWasCancelled :type Boolean))
  (Variables|/Script/CombatGASCompanion.CombatCharacterMovementComponent|SetbThrust (Variables|Default|GetCombat%20Character%20Movement%20Component) false))