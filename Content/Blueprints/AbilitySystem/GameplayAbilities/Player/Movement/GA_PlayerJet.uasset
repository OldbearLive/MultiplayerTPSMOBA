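; Gameplay ability that runs the player's jetpack state on the combat character while its input is held.
; Activation plays the enter-jet montage, whose gameplay event links the jetpack anim layer, triggers a jump and calls JetPressed on the custom movement component.
; Input release calls JetReleased, unlinks the layer and ends the ability; an interrupted or cancelled montage only ends it.
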(event Ability|EventActivateAbility
  (bind _asbp_combat_character (Utilities|Casting|CastToBP_CombatCharacter (Ability|GetAvatarActorfromActorInfo)))
  (Variables|Default|SetAs%20BP%20Combat%20Character _asbp_combat_character)
  (Variables|Default|SetCombat%20Character%20Movement%20Component (Variables|/Script/CombatGASCompanion.CombatCharacter|GetCombatCharacterMovementComponent _asbp_combat_character))
  (|PlayMontageandWaitProxy "None" "/Game/ImportedContent/JetAnimations/EnterJet_Montage.EnterJet_Montage" 1.0 "None" true 1.0 0.0
    (:then
      (Ability|Tasks|WaitGameplayEvent "(TagName=\"Event.Montage.Player.ActiveJet\")" 0 true
        (:EventReceived
          (Default|MCLinkAnimLayer (Variables|Default|GetAs%20BP%20Combat%20Character) "/Game/Blueprints/Character/Animation/ABP_Jetpack.ABP_Jetpack_C")
          ;[1 1 1] JetStateActiveOn Character and AnimLayer is Linked
          (Character|Jump (Variables|Default|GetAs%20BP%20Combat%20Character))
          (Class|CombatCharacterMovementComponent|JetPressed (Variables|Default|GetCombat%20Character%20Movement%20Component))
          ;[1 1 1] Wait Input to DeActivate JetState
          (Ability|Tasks|WaitInputRelease false
            (:OnRelease
              (Class|CombatCharacterMovementComponent|JetReleased (Variables|Default|GetCombat%20Character%20Movement%20Component))
              (Default|MCUnlinkAnimLayer (Variables|Default|GetAs%20BP%20Combat%20Character) "/Game/Blueprints/Character/Animation/ABP_Jetpack.ABP_Jetpack_C")
              (Ability|EndAbility))))))
    (:OnInterrupted
      (Ability|EndAbility :!label _label))
    (:OnCancelled
      (goto _label))))

(event Ability|EventOnEndAbility
  (params (bWasCancelled :type Boolean)))