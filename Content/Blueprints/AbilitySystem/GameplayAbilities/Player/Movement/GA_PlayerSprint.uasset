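; GA_PlayerSprint is a Gameplay Ability that lets the player's CombatCharacter sprint while the input is held.
; On activation it casts the avatar to CombatCharacter, caches its movement component and mesh, commits, and calls SprintPressed on the movement component.
; A WaitInputRelease task then calls SprintReleased and ends the ability when the input is let go.
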(event Ability|EventActivateAbility
  (bind _ascombat_character (Utilities|Casting|CastToCombatCharacter (Ability|GetAvatarActorfromActorInfo)))
  (bind _output_get (Variables|Default|SetAs%20Combat%20Character _ascombat_character))
  (Variables|Default|SetCombat%20Character%20Movement%20Component (Variables|/Script/CombatGASCompanion.CombatCharacter|GetCombatCharacterMovementComponent _output_get))
  (Variables|Default|SetMesh (Variables|/Script/Engine.Character|GetMesh _output_get))
  (Ability|CommitAbility)
  (Class|CombatCharacterMovementComponent|SprintPressed (Variables|Default|GetCombat%20Character%20Movement%20Component))
  (Ability|Tasks|WaitInputRelease false
    (:OnRelease
      (Class|CombatCharacterMovementComponent|SprintReleased (Variables|Default|GetCombat%20Character%20Movement%20Component))
      (Ability|EndAbility))))

(event Ability|EventOnEndAbility
  (params (bWasCancelled :type Boolean)))