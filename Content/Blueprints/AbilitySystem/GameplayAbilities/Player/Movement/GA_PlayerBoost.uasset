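; Player boost ability for jet movement: starts the Jet ability with boost on, or waits for a press if already jetting.
; A re-armed WaitInputPress loop toggles boost, ignoring presses within half a second.
; Boost drives the movement component flag, server state, GE_Boost, rotation settings and an offset camera.
; The JetStop gameplay event or the movement component's end-jet callback ends the ability and clears boost.
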(event Custom|ResetDashPressed
  (bind _timewaited (Ability|Tasks|WaitInputPress false)
    (:then
      (bind _asynctaskproxy (Ability|Tasks|WaitGameplayEvent "(TagName=\"Event.Movement.JetStop\")" 0 true)
        (:then
          (Variables|Default|SetWaitEventTask _asynctaskproxy)
          (EventDispatchers|BindEventtoEndJet (Variables|Default|GetCombat%20Character%20Movement%20Component) (EventDispatchers|CreateEvent :!event Custom|ON%20EndJet)))
        (:EventReceived
          (Ability|EndAbility))))
    (:OnPress
      (if (> _timewaited 0.5)
        (if (Variables|/Script/CombatGASCompanion.CombatCharacterMovementComponent|GetbBoost (Variables|Default|GetCombat%20Character%20Movement%20Component))
          (Variables|/Script/CombatGASCompanion.CombatCharacterMovementComponent|SetbBoost (Variables|Default|GetCombat%20Character%20Movement%20Component) false)
          (Class|CombatCharacter|ServerSetBoosting (Variables|Default|GetAs%20BP%20Combat%20Character) false)
          (Variables|/Script/Engine.Pawn|SetbUseControllerRotationPitch (Variables|Default|GetAs%20BP%20Combat%20Character) false)
          (Variables|/Script/Engine.CharacterMovementComponent|SetbOrientRotationToMovement (Variables|Default|GetCombat%20Character%20Movement%20Component) false)
          (CallFunction|ResetCameraLocation)
          (Ability|RemoveGameplayEffectFromOwnerWithHandle (Variables|Default|GetActive%20GEHandle))
          (else
            (Variables|/Script/CombatGASCompanion.CombatCharacterMovementComponent|SetbBoost (Variables|Default|GetCombat%20Character%20Movement%20Component) true)
            (Class|CombatCharacter|ServerSetBoosting (Variables|Default|GetAs%20BP%20Combat%20Character) true)
            (Variables|/Script/Engine.Pawn|SetbUseControllerRotationPitch (Variables|Default|GetAs%20BP%20Combat%20Character) true)
            (Variables|/Script/Engine.CharacterMovementComponent|SetbOrientRotationToMovement (Variables|Default|GetCombat%20Character%20Movement%20Component) true)
            (CallFunction|SetCameraLocation)
            (bind _returnvalue (Ability|ApplyGameplayEffectToOwner "/Game/Blueprints/AbilitySystem/GameplayEffects/GE_Boost.GE_Boost_C"))
            (Variables|Default|SetActive%20GEHandle _returnvalue)))
        (bind _waiteventtask (Variables|Default|GetWaitEventTask)
          (:then
            (GameplayTasks|EndTask _waiteventtask))
          (:else
            _))
        (CallFunction|ResetDashPressed)
        (else
          (CallFunction|ResetDashPressed))))))

(event Custom|ON%20EndJet
  (Variables|/Script/CombatGASCompanion.CombatCharacterMovementComponent|SetbBoost (Variables|Default|GetCombat%20Character%20Movement%20Component) false)
  (Class|CombatCharacter|ServerSetBoosting (Variables|Default|GetAs%20BP%20Combat%20Character) false)
  (Variables|/Script/Engine.Pawn|SetbUseControllerRotationPitch (Variables|Default|GetAs%20BP%20Combat%20Character) false)
  (Variables|/Script/Engine.CharacterMovementComponent|SetbOrientRotationToMovement (Variables|Default|GetCombat%20Character%20Movement%20Component) false)
  (Ability|RemoveGameplayEffectFromOwnerWithHandle (Variables|Default|GetActive%20GEHandle))
  (Ability|EndAbility))

(event Custom|ResetCameraLocation
  (bind _defaultsocketoffset (Variables|Default|GetDefaultSocketOffset))
  (Default|ClientCameraSetCameraLocation (Variables|Default|GetAs%20BP%20Combat%20Character) (.x _defaultsocketoffset) (.y _defaultsocketoffset) (.z _defaultsocketoffset)))

(event Custom|SetCameraLocation
  (Default|ClientCameraSetCameraLocation (Variables|Default|GetAs%20BP%20Combat%20Character) 1e+02 6e+01 1e+01))

(event Ability|EventActivateAbility
  (bind _asbp_combat_character (Utilities|Casting|CastToBP_CombatCharacter (Ability|GetAvatarActorfromActorInfo)))
  (bind _output_get (Variables|Default|SetAs%20BP%20Combat%20Character _asbp_combat_character))
  (Variables|Default|SetCombat%20Character%20Movement%20Component (Variables|/Script/CombatGASCompanion.CombatCharacter|GetCombatCharacterMovementComponent _asbp_combat_character))
  (Variables|Default|SetDefaultSocketOffset (Variables|/Game/Blueprints/Character/BP_CombatCharacter.BP_CombatCharacter_C|GetDefaulyCameraSocketOffset _output_get))
  (Ability|CommitAbility)
  (bind _returnvalue (Class|CombatCharacterMovementComponent|IsCustomMovementMode (Variables|Default|GetCombat%20Character%20Movement%20Component) "CMOVE_JET"))
  (if (or _returnvalue (GameplayTags|HasMatchingGameplayTag (Ability|GetAbilitySystemComponentfromActorInfo) "(TagName=\"Effects.Movement.Jet\")"))
    (bind _timewaited (Ability|Tasks|WaitInputPress false)
      (:then
        (bind _asynctaskproxy (Ability|Tasks|WaitGameplayEvent "(TagName=\"Event.Movement.JetStop\")" 0 true)
          (:then
            (Variables|Default|SetWaitEventTask _asynctaskproxy)
            (EventDispatchers|BindEventtoEndJet (Variables|Default|GetCombat%20Character%20Movement%20Component) (EventDispatchers|CreateEvent :!event Custom|ON%20EndJet)))
          (:EventReceived
            (Ability|EndAbility))))
      (:OnPress
        (if (> _timewaited 0.5)
          (if (Variables|/Script/CombatGASCompanion.CombatCharacterMovementComponent|GetbBoost (Variables|Default|GetCombat%20Character%20Movement%20Component))
            (Variables|/Script/CombatGASCompanion.CombatCharacterMovementComponent|SetbBoost (Variables|Default|GetCombat%20Character%20Movement%20Component) false)
            (Class|CombatCharacter|ServerSetBoosting (Variables|Default|GetAs%20BP%20Combat%20Character) false)
            (Variables|/Script/Engine.Pawn|SetbUseControllerRotationPitch (Variables|Default|GetAs%20BP%20Combat%20Character) false)
            (Variables|/Script/Engine.CharacterMovementComponent|SetbOrientRotationToMovement (Variables|Default|GetCombat%20Character%20Movement%20Component) false)
            (CallFunction|ResetCameraLocation)
            (Ability|RemoveGameplayEffectFromOwnerWithHandle (Variables|Default|GetActive%20GEHandle))
            (else
              (Variables|/Script/CombatGASCompanion.CombatCharacterMovementComponent|SetbBoost (Variables|Default|GetCombat%20Character%20Movement%20Component) true)
              (Class|CombatCharacter|ServerSetBoosting (Variables|Default|GetAs%20BP%20Combat%20Character) true)
              (Variables|/Script/Engine.Pawn|SetbUseControllerRotationPitch (Variables|Default|GetAs%20BP%20Combat%20Character) true)
              (Variables|/Script/Engine.CharacterMovementComponent|SetbOrientRotationToMovement (Variables|Default|GetCombat%20Character%20Movement%20Component) true)
              (CallFunction|SetCameraLocation)
              (bind _returnvalue_2 (Ability|ApplyGameplayEffectToOwner "/Game/Blueprints/AbilitySystem/GameplayEffects/GE_Boost.GE_Boost_C"))
              (Variables|Default|SetActive%20GEHandle _returnvalue_2)))
          (bind _waiteventtask (Variables|Default|GetWaitEventTask)
            (:then
              (GameplayTasks|EndTask _waiteventtask))
            (:else
              _))
          (CallFunction|ResetDashPressed)
          (else
            (CallFunction|ResetDashPressed)))))
    (else
      (Variables|/Script/CombatGASCompanion.CombatCharacterMovementComponent|SetbBoost (Variables|Default|GetCombat%20Character%20Movement%20Component) true)
      (Class|CombatCharacter|ServerSetBoosting (Variables|Default|GetAs%20BP%20Combat%20Character) true)
      (Abilities|TryActivateAbilitiesbyTag (Ability|GetAbilitySystemComponentfromActorInfo) (GameplayTags|MakeLiteralGameplayTagContainer "(GameplayTags=((TagName=\"Abilities.Movement.Jet\")))") true)
      (Variables|/Script/Engine.Pawn|SetbUseControllerRotationPitch (Variables|Default|GetAs%20BP%20Combat%20Character) true)
      (Variables|/Script/Engine.CharacterMovementComponent|SetbOrientRotationToMovement (Variables|Default|GetCombat%20Character%20Movement%20Component) true)
      (CallFunction|SetCameraLocation)
      (bind _returnvalue_3 (Ability|ApplyGameplayEffectToOwner "/Game/Blueprints/AbilitySystem/GameplayEffects/GE_Boost.GE_Boost_C"))
      (Variables|Default|SetActive%20GEHandle _returnvalue_3)
      (bind _waiteventtask_2 (Variables|Default|GetWaitEventTask)
        (:then
          (GameplayTasks|EndTask _waiteventtask_2))
        (:else
          _))
      (CallFunction|ResetDashPressed))))

(event Ability|EventOnEndAbility
  (params (bWasCancelled :type Boolean))
  (Variables|/Script/CombatGASCompanion.CombatCharacterMovementComponent|SetbBoost (Variables|Default|GetCombat%20Character%20Movement%20Component) false)
  (Class|CombatCharacter|ServerSetBoosting (Variables|Default|GetAs%20BP%20Combat%20Character) false)
  (Variables|/Script/Engine.Pawn|SetbUseControllerRotationPitch (Variables|Default|GetAs%20BP%20Combat%20Character) false)
  (Variables|/Script/Engine.CharacterMovementComponent|SetbOrientRotationToMovement (Variables|Default|GetCombat%20Character%20Movement%20Component) false)
  (Ability|RemoveGameplayEffectFromOwnerWithHandle (Variables|Default|GetActive%20GEHandle))
  (CallFunction|ResetCameraLocation))