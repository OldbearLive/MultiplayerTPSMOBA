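; Base player gameplay ability that fires a projectile from the combat character's active ranged weapon.
; A target-data-under-mouse task supplies the aim point, using the impact point on a hit or the trace end otherwise.
; With a valid weapon, it commits, spawns the projectile at the weapon's socket, calls Fire and plays the fire montage.
; The server ends the ability right after starting the montage, which keeps playing.
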(event Custom|MC_PlayMontage
  (params (MontageToPlay :type Anim%20Montage%20Object%20Reference) (StartSection :type Name)))

(event Custom|Server_PlayMontage
  (params (MontageToPlay :type Anim%20Montage%20Object%20Reference) (StartSection :type Name))
  (CallFunction|MCPlayMontage MontageToPlay StartSection))

(event Ability|EventActivateAbility
  (bind _datahandle (|TargetDataUnderMouse)
    (:ValidData
      (Variables|Default|SetBlocking%20Hit (.bBlockingHit (Collision|BreakHitResult (Ability|TargetData|GetHitResultfromTargetData _datahandle))))
      (Variables|Default|SetProjectileTargetLocation (.ImpactPoint (Collision|BreakHitResult (Ability|TargetData|GetHitResultfromTargetData _datahandle))))
      (Variables|Default|SetTrace%20End (.TraceEnd (Collision|BreakHitResult (Ability|TargetData|GetHitResultfromTargetData _datahandle))))
      (bind _asbp_combat_character (Utilities|Casting|CastToBP_CombatCharacter (Ability|GetAvatarActorfromActorInfo)))
      (Variables|Default|SetAs%20BP%20Combat%20Character _asbp_combat_character)
      (Utilities|IsValid (Utilities|Array|Get(acopy) (Variables|/Script/CombatGASCompanion.CombatCharacter|GetCombatRangedWeaponsArray (Variables|Default|GetAs%20BP%20Combat%20Character)) (Variables|/Script/CombatGASCompanion.CombatCharacter|GetActiveWeaponIndex (Variables|Default|GetAs%20BP%20Combat%20Character)))
        (:Is%20Valid
          (Ability|CommitAbility)
          (Variables|Default|SetSpawnTransform (Math|Transform|MakeTransform (Transformation|GetSocketLocation (Variables|/Script/CombatGASCompanion.CombatRangedWeapon|GetWeaponMesh (Utilities|Array|Get(acopy) (Variables|/Script/CombatGASCompanion.CombatCharacter|GetCombatRangedWeaponsArray (Variables|Default|GetAs%20BP%20Combat%20Character)) (Variables|/Script/CombatGASCompanion.CombatCharacter|GetActiveWeaponIndex (Variables|Default|GetAs%20BP%20Combat%20Character)))) "ProjectileSocket") (.Rotation (Math|Transform|BreakTransform (Variables|Default|GetSpawnTransform))) (.Scale (Math|Transform|BreakTransform (Variables|Default|GetSpawnTransform)))))
          (if (Variables|Default|GetBlocking%20Hit)
            (Class|CombatProjectileAbility|SpawnProjectile (Variables|Default|GetProjectileTargetLocation))
            (else
              (Class|CombatProjectileAbility|SpawnProjectile (Variables|Default|GetTrace%20End))))
          (Class|CombatRangedWeapon|Fire (Utilities|Array|Get(acopy) (Variables|/Script/CombatGASCompanion.CombatCharacter|GetCombatRangedWeaponsArray (Variables|Default|GetAs%20BP%20Combat%20Character)) (Variables|/Script/CombatGASCompanion.CombatCharacter|GetActiveWeaponIndex (Variables|Default|GetAs%20BP%20Combat%20Character))))
          (|PlayMontageandWaitProxy "None" (.FireMontage (Utilities|Struct|BreakWeaponProperties (Variables|/Script/CombatGASCompanion.CombatRangedWeapon|GetWeaponPropertiesStructure (Utilities|Array|Get(acopy) (Variables|/Script/CombatGASCompanion.CombatCharacter|GetCombatRangedWeaponsArray (Variables|Default|GetAs%20BP%20Combat%20Character)) (Variables|/Script/CombatGASCompanion.CombatCharacter|GetActiveWeaponIndex (Variables|Default|GetAs%20BP%20Combat%20Character)))))) 1.0 "RifleAim" false 1.0 0.0
            (:then
              (if (Networking|IsServer)
                (Ability|EndAbility)))))
        (:Is%20Not%20Valid
          (Ability|EndAbility))))))

(event Ability|EventOnEndAbility
  (params (bWasCancelled :type Boolean)))