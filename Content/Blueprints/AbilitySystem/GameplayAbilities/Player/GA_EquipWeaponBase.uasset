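; Base Gameplay Ability that equips a ranged weapon into an inventory slot on the combat character.
; On activation it destroys any weapon in that slot, then spawns the configured class and snaps it to a mesh socket.
; The server registers the new weapon in the inventory and ends the ability.
; An in-range but empty slot ends the ability without spawning.
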(event Ability|EventActivateAbility
  ;[1 1 1] ActivateAbility Store Combat CharacterRef
  (bind _asbp_combat_character (Utilities|Casting|CastToBP_CombatCharacter (Ability|GetAvatarActorfromActorInfo))
    (:then
      (Variables|Default|SetAs%20BP%20Combat%20Character _asbp_combat_character)
      ;[1 1 1] Check to see if Weapon Inventory has a valid item at the inventory index
      (if (Utilities|Array|IsValidIndex (Variables|/Script/CombatGASCompanion.CombatCharacter|GetCombatRangedWeaponsArray (Variables|Default|GetAs%20BP%20Combat%20Character)) (Variables|Default|GetInventorySlot))
        (Utilities|IsValid (Utilities|Array|Get(acopy) (Variables|/Script/CombatGASCompanion.CombatCharacter|GetCombatRangedWeaponsArray (Variables|Default|GetAs%20BP%20Combat%20Character)) (Variables|Default|GetInventorySlot))
          (:Is%20Valid
            (Actor|DestroyActor (Utilities|Array|Get(acopy) (Variables|/Script/CombatGASCompanion.CombatCharacter|GetCombatRangedWeaponsArray (Variables|Default|GetAs%20BP%20Combat%20Character)) (Variables|Default|GetInventorySlot)))
            (bind _spawnedactor (|SpawnActor :Class (Variables|Default|GetWeaponClass) :Instigator _asbp_combat_character :!label _label)
              (:Success
                (bind _asbp_range_weapon_base (Utilities|Casting|CastToBP_RangeWeaponBase _spawnedactor)
                  (:then
                    (Variables|Default|SetAs%20BP%20Range%20Weapon%20Base _asbp_range_weapon_base)
                    (Transformation|AttachComponentToComponent (Variables|Default|GetAs%20BP%20Range%20Weapon%20Base) (Variables|/Script/Engine.Character|GetMesh (Variables|Default|GetAs%20BP%20Combat%20Character)) (Variables|Default|GetEquipAttachSocket) "SnapToTarget" "SnapToTarget" "SnapToTarget" true)
                    (if (Networking|IsServer)
                      (Default|ServerAddWeapontoInventory (Variables|Default|GetAs%20BP%20Combat%20Character) (Variables|Default|GetInventorySlot) (Variables|Default|GetAs%20BP%20Range%20Weapon%20Base))
                      (Ability|EndAbility)))
                  (:CastFailed
                    (Ability|EndAbility :!label _label_2))))
              (:DidNotSpawn
                (goto _label_2))))
          (:Is%20Not%20Valid
            (Ability|EndAbility)))
        (else
          (goto _label))))
    (:CastFailed
      (Ability|EndAbility))))