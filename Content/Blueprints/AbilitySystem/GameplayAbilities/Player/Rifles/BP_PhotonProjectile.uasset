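; Photon rifle projectile for the player's ability system that deals physical damage to what it hits.
; On box overlap with anything but its owner, it stops the tracer tail and calls OnOverlap.
; Targets with an ability system receive the damage effect spec with a fixed set-by-caller magnitude, unless the hit component is tagged Armor.
; It then disables collision, removes its arrow and destroys itself after a short delay.
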(event OnComponentBeginOverlap(BoxComponent)
  (params (OverlappedComponent :type Primitive%20Component%20Object%20Reference) (OtherActor :type Actor%20Object%20Reference) (OtherComp :type Primitive%20Component%20Object%20Reference) (OtherBodyIndex :type Integer) (bFromSweep :type Boolean) (SweepResult :type Hit%20Result%20Structure%20%28by%20ref%29))
  (bind _returnvalue (Ability|GetAbilitySystemComponent OtherActor))
  (if (not (== OtherActor (Components|GetOwner)))
    (bind _tracertailcomponent (Variables|Default|GetTracerTailComponent)
      (:then
        (Components|Activation|Deactivate _tracertailcomponent))
      (:else
        _))
    (Class|CombatProjectile|OnOverlap OtherActor)
    (if (Components|ComponentHasTag OtherComp "Armor")
      _
      (else
        (Utilities|IsValid _returnvalue
          (:Is%20Valid
            (bind _returnvalue_2 (Ability|GameplayEffect|AssignTagSetbyCallerMagnitude (Variables|Default|GetDamageEffectSpecHandle) "(TagName=\"Damage.Physical\")" 3e+02))
            (GameplayEffects|ApplyGameplayEffectSpecToSelf _returnvalue _returnvalue_2))
          (:Is%20Not%20Valid
            _))))
    (Collision|SetCollisionEnabled (Variables|Default|GetBoxComponent) "NoCollision")
    (Components|DestroyComponent (Variables|Default|GetArrow))
    (Utilities|FlowControl|Delay 2.0)
    (Actor|DestroyActor)))

(event EventBeginPlay
  (|CallParentFunction))

(fn ConstructionScript)