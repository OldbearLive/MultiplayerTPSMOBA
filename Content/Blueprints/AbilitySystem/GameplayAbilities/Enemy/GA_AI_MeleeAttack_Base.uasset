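; Base gameplay ability for AI melee attacks that plays a random montage from the avatar's combat interface.
; While waiting for the montage's tagged event, it focuses the AI on its combat target with a temporary rotation rate.
; The event fires a gameplay cue, damages non-friendly live players around the combat socket, draws debug output, then restores focus and rotation.
; Montage completion, interruption or cancellation ends the ability without that restore.
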(event Ability|EventActivateAbility
  (bind _returnvalue (Ability|GetAvatarActorfromActorInfo))
  (bind _returnvalue_2 (Ability|GetAvatarActorfromActorInfo))
  (bind _returnvalue_3 (Ability|GetAvatarActorfromActorInfo))
  (bind _ascombat_interface (Utilities|Casting|CastToCombatInterface (Ability|GetAvatarActorfromActorInfo)))
  (bind _returnvalue_4 (Class|CombatInterface|GetAttackMontages _ascombat_interface))
  (Variables|Default|SetTaggedMontage (Utilities|Array|Get(acopy) _returnvalue_4 (Math|Random|RandomIntegerinRange 0 (- (Utilities|Array|Length _returnvalue_4) 1))))
  (|PlayMontageandWaitProxy "None" (.Montage (Utilities|Struct|BreakTaggedMontage (Variables|Default|GetTaggedMontage))) 1.0 "None" false 1.0 0.0
    (:then
      (Ability|Tasks|WaitGameplayEvent (.MontageTag (Utilities|Struct|BreakTaggedMontage (Variables|Default|GetTaggedMontage))) 0
        (:then
          (bind _returnvalue_5 (Class|CombatInterface|GetCombatTarget(Message) _returnvalue_2))
          (AI|SetFocus (AI|GetAIController _returnvalue_2) _returnvalue_5)
          (bind _ascharacter (Utilities|Casting|CastToCharacter _returnvalue_2))
          (Variables|Default|SetPreviousRotationRate (Variables|/Script/Engine.CharacterMovementComponent|GetRotationRate (Variables|/Script/Engine.Character|GetCharacterMovement _ascharacter)))
          (Variables|/Script/Engine.CharacterMovementComponent|SetRotationRate (Variables|/Script/Engine.Character|GetCharacterMovement _ascharacter) (Variables|Default|GetFocusRotationRate)))
        (:EventReceived
          (bind _returnvalue_6 (Class|CombatInterface|GetCombatSocketLocation(Message) _returnvalue))
          (Rendering|Debug|DrawDebugSphere _returnvalue_6 (Variables|Default|GetRadius) 12 "(R=1.000000,G=0.000000,B=0.008526,A=1.000000)" 2.0 5.0)
          (Class|GameplayAbility|ExecuteGameplayCuewithParams (Variables|Default|GetSoundAndEffectsGCTag) (Ability|GameplayCue|MakeGameplayCueParameters :Location _returnvalue_6 :Instigator (Ability|GetAvatarActorfromActorInfo)))
          (bind _overlappingactors (Class|CombatBlueprintFunctionLibrary|GetLivePlayersWithinRadius _returnvalue (Utilities|Array|MakeArray _returnvalue) (Variables|Default|GetRadius) _returnvalue_6))
          (for _array_element _overlappingactors
            (if (Class|CombatBlueprintFunctionLibrary|IsNotFriend (Ability|GetAvatarActorfromActorInfo) _array_element)
              (Class|CombatDamageGameplayAbility|CauseDamage _array_element)
              (Development|PrintString (Utilities|GetObjectName _array_element))))
          (AI|ClearFocus (AI|GetAIController _returnvalue_3))
          (bind _ascharacter_2 (Utilities|Casting|CastToCharacter _returnvalue_3))
          (Variables|/Script/Engine.CharacterMovementComponent|SetRotationRate (Variables|/Script/Engine.Character|GetCharacterMovement _ascharacter_2) (Variables|Default|GetPreviousRotationRate)))))
    (:OnCompleted
      (Ability|EndAbility :!label _label))
    (:OnInterrupted
      (goto _label))
    (:OnCancelled
      (goto _label))))

(event Ability|EventOnEndAbility
  (params (bWasCancelled :type Boolean)))