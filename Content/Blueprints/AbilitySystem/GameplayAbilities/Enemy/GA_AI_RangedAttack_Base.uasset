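; Base enemy AI ranged attack ability that fires a series of projectiles at the combat target during a tagged montage.
; On activation it focuses the AI on the target and swaps the character's rotation rate, saving the previous value.
; The montage's gameplay event starts timed shots, each playing an effects cue at the fire socket, then spawning a projectile after a delay.
; It ends after the last shot's delays or when the montage finishes or is interrupted.
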(event Ability|EventActivateAbility
  (bind _returnvalue (Ability|GetAvatarActorfromActorInfo))
  (bind _projectilefiresocket (Variables|Default|GetProjectileFireSocket))
  (bind _taggedmontage (Variables|Default|GetTaggedMontage))
  (bind (_montage _montagetag) (Utilities|Struct|BreakTaggedMontage _taggedmontage))
  (|PlayMontageandWaitProxy "None" _montage 1.0 "None" false 1.0 0.0
    (:then
      (Ability|Tasks|WaitGameplayEvent _montagetag 0
        (:then
          (bind _returnvalue_2 (Class|CombatInterface|GetCombatTarget(Message) _returnvalue))
          (AI|SetFocus (AI|GetAIController _returnvalue) _returnvalue_2)
          (bind _ascharacter (Utilities|Casting|CastToCharacter _returnvalue))
          (Variables|Default|SetPreviousRotationRate (Variables|/Script/Engine.CharacterMovementComponent|GetRotationRate (Variables|/Script/Engine.Character|GetCharacterMovement _ascharacter)))
          (Variables|/Script/Engine.CharacterMovementComponent|SetRotationRate (Variables|/Script/Engine.Character|GetCharacterMovement _ascharacter) (Variables|Default|GetFocusRotationRate)))
        (:EventReceived
          (|RepeatAction (Variables|Default|GetTimeBetween%20Shots) (Variables|Default|GetTotal%20Shots)
            (:OnPerformAction
              (for _array_element (Actor|GetComponentsByClass (Ability|GetAvatarActorfromActorInfo) "/Script/Engine.SkeletalMeshComponent")
                (if (Transformation|DoesSocketExist _array_element _projectilefiresocket)
                  (Variables|Default|SetSpawnTransform (Math|Transform|MakeTransform (Transformation|GetSocketLocation _array_element _projectilefiresocket) (.rotation (Variables|Default|GetSpawnTransform)) (.scale (Variables|Default|GetSpawnTransform))))
                  (bind _returnvalue_3 (Class|CombatInterface|GetCombatTarget(Message) (Ability|GetAvatarActorfromActorInfo)))
                  (Class|GameplayAbility|ExecuteGameplayCuewithParams (Variables|Default|GetSoundAndEffectsGCTag) (Ability|GameplayCue|MakeGameplayCueParameters :Location (Transformation|GetSocketLocation _array_element _projectilefiresocket) :Instigator (Ability|GetAvatarActorfromActorInfo) :SourceObject _returnvalue_3))
                  (Ability|Tasks|WaitDelay (Variables|Default|GetProjectileSpawnWaitAfterGC)
                    (:OnFinish
                      (Class|CombatProjectileAbility|SpawnProjectile (Transformation|GetActorLocation _returnvalue_3)))))))
            (:OnFinished
              (Ability|Tasks|WaitDelay (Variables|Default|GetProjectileSpawnWaitAfterGC)
                (:OnFinish
                  (Ability|Tasks|WaitDelay (Math|Float|SafeDivide (Variables|Default|GetProjectileSpawnWaitAfterGC) 2.0)
                    (:OnFinish
                      (Ability|EndAbility))))))))))
    (:OnCompleted
      (Ability|EndAbility :!label _label))
    (:OnInterrupted
      (goto _label))
    (:OnCancelled
      (goto _label))))

(event Ability|EventOnEndAbility
  (params (bWasCancelled :type Boolean)))