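; Enemy death gameplay ability that applies GE_Death and plays the walker death montage on a TEST_enemy avatar.
; Once the montage starts, it disables mesh collision and waits for a single Event.DeathEvent gameplay event.
; That event calls MC_PauseAnim to freeze animation and skeleton updates, holding the pose, then ends the ability.
; The effect-removal node is unconnected, so this ability never removes GE_Death.
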(event Custom|MC_PauseAnim
  (bind _enemy (Variables|Default|GetEnemy))
  (bind _mesh (Variables|/Script/Engine.Character|GetMesh _enemy))
  (Variables|/Script/Engine.SkeletalMeshComponent|SetbPauseAnims _mesh true)
  (Variables|/Script/Engine.SkeletalMeshComponent|SetbNoSkeletonUpdate _mesh true))

(event Ability|EventActivateAbility
  (bind _returnvalue (Ability|ApplyGameplayEffectToOwner "/Game/Blueprints/AbilitySystem/GameplayEffects/GE_Death.GE_Death_C"))
  (Variables|Default|SetActive%20GEHandle _returnvalue)
  (bind _astest_enemy (Utilities|Casting|CastToTEST_enemy (Ability|GetAvatarActorfromActorInfo)))
  (Variables|Default|SetEnemy _astest_enemy)
  (|PlayMontageandWaitProxy "None" "/Game/ImportedContent/Walker_2/Walker_Death_Montage.Walker_Death_Montage" 1.0 "None" false 1.0 0.0
    (:then
      (Ability|Async|WaitGameplayEventToActor (Ability|GetAvatarActorfromActorInfo) "(TagName=\"Event.DeathEvent\")" true
        (:then
          (Collision|SetCollisionEnabled (Variables|/Script/Engine.Character|GetMesh _astest_enemy) "NoCollision"))
        (:EventReceived
          (CallFunction|MCPauseAnim)
          (Ability|EndAbility))))))

(event Ability|EventOnEndAbility
  (params (bWasCancelled :type Boolean)))