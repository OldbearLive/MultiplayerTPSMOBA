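; Base gameplay ability in the enemy folder that lets a BP_Walker fire a projectile toward the cursor, apparently while possessed.
; On activation it commits, plays the tagged montage and waits for that montage's gameplay event.
; The event triggers a target-data-under-mouse task, and SpawnProjectile receives the impact point, or the trace end without a blocking hit.
; The spawn transform takes its location from the mesh's ranged-combat socket, and the ability ends after spawning.
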(event Ability|EventActivateAbility
  (bind _taggedmontage (Variables|Default|GetTaggedMontage))
  (bind (_montage _montagetag) (Utilities|Struct|BreakTaggedMontage _taggedmontage))
  (bind _asbp_walker (Utilities|Casting|CastToBP_Walker (Ability|GetAvatarActorfromActorInfo)))
  (Variables|Default|SetAs%20BP%20Walker _asbp_walker)
  (Ability|CommitAbility)
  (|PlayMontageandWaitProxy "None" _montage 1.0 "" false 1.0 0.0
    (:then
      (Ability|Tasks|WaitGameplayEvent _montagetag (Variables|Default|GetAs%20BP%20Walker)
        (:EventReceived
          (bind _datahandle (|TargetDataUnderMouse)
            (:ValidData
              (Variables|Default|SetBlocking%20Hit (.bBlockingHit (Collision|BreakHitResult (Ability|TargetData|GetHitResultfromTargetData _datahandle))))
              (Variables|Default|SetProjectileTargetLocation (.ImpactPoint (Collision|BreakHitResult (Ability|TargetData|GetHitResultfromTargetData _datahandle))))
              (Variables|Default|SetTrace%20End (.TraceEnd (Collision|BreakHitResult (Ability|TargetData|GetHitResultfromTargetData _datahandle))))
              (Variables|Default|SetSpawnTransform (Math|Transform|MakeTransform (Transformation|GetSocketLocation (Variables|/Script/Engine.Character|GetMesh (Variables|Default|GetAs%20BP%20Walker)) (Variables|Default|GetRangedCombatSocketName)) (.Rotation (Math|Transform|BreakTransform (Variables|Default|GetSpawnTransform))) (.Scale (Math|Transform|BreakTransform (Variables|Default|GetSpawnTransform)))))
              (if (Variables|Default|GetBlocking%20Hit)
                (Class|CombatProjectileAbility|SpawnProjectile (Variables|Default|GetProjectileTargetLocation))
                (else
                  (Class|CombatProjectileAbility|SpawnProjectile (Variables|Default|GetTrace%20End))))
              (Ability|EndAbility))))))))

(event Ability|EventOnEndAbility
  (params (bWasCancelled :type Boolean)))