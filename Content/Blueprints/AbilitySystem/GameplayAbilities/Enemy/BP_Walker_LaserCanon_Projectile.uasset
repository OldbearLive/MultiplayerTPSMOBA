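; Projectile for the Walker enemy's laser cannon ability, extending a parent projectile class with its own impact and cleanup.
; On begin play it sets the Arrow as the projectile movement's interpolated component.
; A box overlap with any actor except the owner calls OnOverlap, disables box collision and stops simulation.
; When movement stops, it removes the sphere, waits briefly, then deactivates the tracer tail and destroys itself.
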(event OnProjectileStop(ProjectileMovementComponent)
  (params (ImpactResult :type Hit%20Result%20Structure%20%28by%20ref%29))
  (Components|DestroyComponent (Variables|Default|GetSphere))
  (Utilities|FlowControl|Delay 1.0)
  (bind _tracertailcomponent (Variables|Default|GetTracerTailComponent)
    (:then
      (Components|Activation|Deactivate _tracertailcomponent))
    (:else
      _))
  (Actor|DestroyActor))

(event OnComponentBeginOverlap(BoxComponent)
  (params (OverlappedComponent :type Primitive%20Component%20Object%20Reference) (OtherActor :type Actor%20Object%20Reference) (OtherComp :type Primitive%20Component%20Object%20Reference) (OtherBodyIndex :type Integer) (bFromSweep :type Boolean) (SweepResult :type Hit%20Result%20Structure%20%28by%20ref%29))
  (if (not (== OtherActor (Components|GetOwner)))
    (Class|CombatProjectile|OnOverlap OtherActor)
    (Collision|SetCollisionEnabled (Variables|Default|GetBoxComponent) "NoCollision")
    (Game|Components|ProjectileMovement|StopSimulating (Variables|Default|GetProjectileMovementComponent) SweepResult)))

(event EventBeginPlay
  (|CallParentFunction)
  (Game|Components|ProjectileMovement|Interpolation|SetInterpolatedComponent (Variables|Default|GetProjectileMovementComponent) (Variables|Default|GetArrow)))

(fn ConstructionScript)