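; Base gameplay ability for equipping a ranged weapon on a combat character.
; It plays the equip montage and waits once for the equip gameplay event, then spawns the weapon class with the avatar as instigator and snaps it to a socket on the character mesh.
; With authority, it then links the weapon anim layer through the character's server call.
; The EndAbility calls are unwired, so the graph never ends the ability itself.
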(event Ability|EventActivateAbility
  (|PlayMontageandWaitProxy "None" (Variables|Default|GetEquipMontage) 1.0 "None" true 1.0 0.0
    (:then
      (Ability|Tasks|WaitGameplayEvent (Variables|Default|GetEquipEventTag) 0 true false
        (:EventReceived
          (bind _asbp_combat_character (Utilities|Casting|CastToBP_CombatCharacter (Ability|GetAvatarActorfromActorInfo)))
          (Variables|Default|SetAs%20BP%20Combat%20Character _asbp_combat_character)
          (bind _spawnedactor (|SpawnActor :Class (Variables|Default|GetWeaponClass) :Instigator _asbp_combat_character)
            (:Success
              (bind _ascombat_ranged_weapon (Utilities|Casting|CastToCombatRangedWeapon _spawnedactor))
              (Transformation|AttachComponentToComponent _ascombat_ranged_weapon (Variables|/Script/Engine.Character|GetMesh _asbp_combat_character) (Variables|Default|GetAttachSocketName) "SnapToTarget" "SnapToTarget" "SnapToTarget" true)
              (Ability|HasAuthority
                (:True
                  (Default|ServerLinkAnimLayer (Variables|Default|GetAs%20BP%20Combat%20Character) (Variables|Default|GetAnimclassToLink)))))))))))

(event Ability|EventOnEndAbility
  (params (bWasCancelled :type Boolean)))