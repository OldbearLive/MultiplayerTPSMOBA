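; BP_CombatCharacter is the multiplayer combat character, using GAS for weapon equipping and replicating ranged weapon state.
; Server-to-multicast RPC pairs link anim layers, fill the weapon inventory and set active weapon fire properties.
; Possession disables client input; Client_EquipWeapons activates every granted GA_EquipWeaponBase ability, while Server_EquipWeapons sets the equipped flag for the AnimBP.
; Remote players get an overhead stats widget, cleared for the local player.
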(event Custom|Client_DisableInput
  (params (PlayerController :type Player%20Controller%20Object%20Reference))
  ;[1 1 1] Disable Input after posession
  (Input|DisableInput PlayerController))

(event Custom|MC_LinkAnimLayer
  (params (InClass :type Anim%20Instance%20Class%20Reference))
  ;[1 1 1] Multicast RPC to Link Anim Layer
  (Components|SkeletalMesh|AnimationBlueprintLinking|LinkAnimClassLayers (Variables|Character|GetMesh) InClass))

(event Custom|Server_SelectWeapon
  (params (InventoryIndex :type Integer) (WeaponProperties :type Weapon%20Properties%20Structure))
  (CallFunction|MCSelectWeapon InventoryIndex WeaponProperties))

(event Custom|ServerSetMPStatsBar
  (params (MultiplayerStatsBar :type WBP%20Multiplayer%20Stats%20Object%20Reference))
  (CallFunction|MCSetMPStatsBar MultiplayerStatsBar))

(event Custom|Server_EquipWeapons
  ;[1 1 1 1 74] Called From CombatGamemode Which Equips all default Weapons
  ;;[1 0 0] ServerSet ReplicatedVariable to read in AnimBP
  (Variables|Default|SetbIsWeaponEquipped true))

(event Custom|MC_SelectWeapon
  (params (InventoryIndex :type Integer) (WeaponProperties :type Weapon%20Properties%20Structure))
  (Weapon|ServerSetReplicatedWeaponVariables InventoryIndex WeaponProperties))

(event Custom|Client_EquipWeapons
  (bind _self self)
  (bind _returnvalue (Ability|GetAbilitySystemComponent _self))
  ;[1 1 1 1 74] Called From CombatGamemode Which Equips all default Weapons
  (Utilities|IsValid _returnvalue
    (:Is%20Valid
      (bind _outabilityhandles (Class|AbilitySystemComponent|GetAllAbilities _returnvalue))
      (for _array_element _outabilityhandles
        (if (.bSuccess (Utilities|Casting|CastToGA_EquipWeaponBase (.ReturnValue (Ability|GameplayAbility|GetGameplayAbilityfromSpecHandle _returnvalue _array_element))))
          (Abilities|TryActivateAbilitybyClass _returnvalue (Utilities|GetClass (.ReturnValue (Ability|GameplayAbility|GetGameplayAbilityfromSpecHandle _returnvalue _array_element))) true)
          (Utilities|IsValid (Variables|Default|GetMultiplayerStatsBar)))))))

(event Custom|Server_LinkAnimLayer
  (params (InClass :type Anim%20Instance%20Class%20Reference))
  ;[1 1 1] Multicast RPC to Link Anim Layer
  (CallFunction|MCLinkAnimLayer InClass))

(event Custom|MC_SetMPStatsBar
  (params (MultiplayerStatsBar :type WBP%20Multiplayer%20Stats%20Object%20Reference)))

(event Custom|MCAddWeaponToInventory
  (params (InventoryIndex :type Integer) (Item :type BP%20Range%20Weapon%20Base%20Object%20Reference%20%28by%20ref%29))
  (Weapon|ServerAddWeapontoInventoryFunc InventoryIndex Item))

(event Custom|ServerAddWeaponToInventory
  (params (InventoryIndex :type Integer) (Item :type BP%20Range%20Weapon%20Base%20Object%20Reference%20%28by%20ref%29))
  (CallFunction|MCAddWeapontoInventory InventoryIndex Item))

(event Custom|AddMultiplayerWidget
  (if (Pawn|IsLocallyControlled)
    (UserInterface|SetWidget (Variables|Default|GetRemoteStatsBar) 0)
    (else
      (bind _aswbp_multiplayer_stats (Utilities|Casting|CastToWBP_MultiplayerStats (UserInterface|GetWidget (Variables|Default|GetRemoteStatsBar))))
      (Variables|Default|SetMultiplayerStatsBar _aswbp_multiplayer_stats)
      (Utilities|IsValid (Variables|Default|GetMultiplayerStatsBar)
        (:Is%20Valid
          (Class|CombatUserWidget|SetWidgetController (Variables|Default|GetMultiplayerStatsBar) self))))))

(event EventBeginPlay)

(event EventPossessed
  (params (NewController :type Controller%20Object%20Reference))
  ;[1 1 1] Disable Input after posession
  (CallFunction|ClientDisableInput (.AsPlayer%20Controller (Utilities|Casting|CastToPlayerController NewController))))

(event EventTick
  (params (DeltaSeconds :type Float%20%28single-precision%29)))

(fn ConstructionScript)

(fn ServerAddWeapontoInventoryFunc
  (params (Index :type Integer) (Item :type BP%20Range%20Weapon%20Base%20Object%20Reference%20%28by%20ref%29))
  (Utilities|Array|SetArrayElem (Variables|Default|GetCombatRangedWeaponsArray) Index Item true)
  (return))

(fn ServerSetReplicatedWeaponVariables
  (params (InventoryIndex :type Integer) (WeaponProperties :type Weapon%20Properties%20Structure))
  (bind (_displayname _bisautofire _bisshotgun _firerate) (Utilities|Struct|BreakWeaponProperties WeaponProperties))
  (Variables|Default|SetActiveWeaponIndex InventoryIndex)
  (Variables|Weapon|WeaponProperties|SetIs%20Auto%20Fire _bisautofire)
  (Variables|Weapon|WeaponProperties|SetIs%20Shotgun _bisshotgun)
  (Variables|Weapon|WeaponProperties|SetFire%20Rate _firerate)
  (return))

(fn GetCombatSocketLocation
  (return "0, 0, 0"))

(fn GetStatusWidgetLocation
  (return (Transformation|GetWorldLocation (Variables|Default|GetMultiplayerStatusWidgetTransform))))

(fn GetHitReactMontage
  (return "/Game/Blueprints/Character/Animation/HitReactions/HitReactionMontage.HitReactionMontage"))