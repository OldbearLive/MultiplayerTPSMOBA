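; BP_CombatGamemode is the game mode that spawns players at numbered player starts and equips them for solo or arena combat.
; As players join, it collects their controllers and reads the expected player count and solo flag from CombatSteamGameInstance.
; Solo games spawn immediately, while arena games wait until every expected player has joined, then spawn each by join index after a short delay.
; After a further delay, each pawn gets input enabled, client-side weapons and the multiplayer widget.
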(event Custom|EquipDefaultWeapons
  (Utilities|FlowControl|Delay 0.5)
  (for _array_element (Variables|Default|GetAllNetPlayerControllers)
    (bind _asbp_combat_character (Utilities|Casting|CastToBP_CombatCharacter (Pawn|GetControlledPawn _array_element)))
    (Default|EnableAllInput _array_element)
    (Default|ClientEquipWeapons _asbp_combat_character)
    (Default|AddMultiplayerWidget _asbp_combat_character)))

(event EventHandleStartingNewPlayer
  (params (NewPlayer :type Player%20Controller%20Object%20Reference))
  (bind _allnetplayercontrollers (Variables|Default|GetAllNetPlayerControllers))
  (bind _output (Utilities|Array|Get(acopy) _allnetplayercontrollers))
  (bind _asbp_combat_player_controller (Utilities|Casting|CastToBP_CombatPlayerController NewPlayer))
  (Utilities|Array|Add (Variables|Default|GetAllNetPlayerControllers) _asbp_combat_player_controller)
  (bind _ascombat_steam_game_instance (Utilities|Casting|CastToCombatSteamGameInstance (Game|GetGameInstance)))
  (Variables|Default|SetNumOfExpectedPlayers (Variables|/Game/Blueprints/Multiplayer/CombatSteamGameInstance.CombatSteamGameInstance_C|GetNumof%20Connected%20Players _ascombat_steam_game_instance))
  (if (Variables|/Game/Blueprints/Multiplayer/CombatSteamGameInstance.CombatSteamGameInstance_C|GetisSoloGame _ascombat_steam_game_instance)
    ;[1 1 1] SOLO GAME
    (Variables|Default|SetNumOfExpectedPlayers 1)
    (Class|GameModeBase|RestartPlayeratPlayerStart _output (Class|GameModeBase|FindPlayerStart _output "0"))
    (CallFunction|EquipDefaultWeapons)
    (else
      ;[1 1 1] Arena
      (if (== (Variables|Default|GetNumOfExpectedPlayers) (Utilities|Array|Length (Variables|Default|GetAllNetPlayerControllers)))
        (Utilities|FlowControl|Delay 2.0)
        (for (_array_element _array_index) (Variables|Default|GetAllNetPlayerControllers)
          (Class|GameModeBase|RestartPlayeratPlayerStart _array_element (Class|GameModeBase|FindPlayerStart _array_element (Utilities|String|ToString(Integer) _array_index))))
        (CallFunction|EquipDefaultWeapons)))))

(fn ConstructionScript)