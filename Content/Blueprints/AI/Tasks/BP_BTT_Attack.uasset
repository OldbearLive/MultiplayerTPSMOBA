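; Behavior tree task that makes an AI pawn attack its combat target through the Gameplay Ability System.
; It reads the target from a blackboard key, passes it to the pawn via a combat target message, then activates abilities matching a configurable tag.
; On activation it waits a set duration before finishing successfully, rather than tracking the ability's end, and fails if the target is invalid or activation fails.
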(event EventReceiveExecuteAI
  (params (OwnerController :type AI%20Controller%20Object%20Reference) (ControlledPawn :type Pawn%20Object%20Reference))
  (bind _combattargetselector (Variables|Default|GetCombatTargetSelector))
  (bind _returnvalue (AI|BehaviorTree|GetBlackboardValueasActor _combattargetselector))
  (Utilities|IsValid _returnvalue
    (:Is%20Valid
      (Class|CombatInterface|SetCombatTarget(Message) ControlledPawn _returnvalue)
      (bind _returnvalue_2 (Abilities|TryActivateAbilitiesbyTag (Ability|GetAbilitySystemComponent ControlledPawn) (GameplayTags|MakeGameplayTagContainerfromTag (Variables|Default|GetAbilitiyTag)) true))
      (if _returnvalue_2
        (Utilities|FlowControl|Delay (Variables|Default|GetAbilityDuration))
        (AI|BehaviorTree|FinishExecute true)
        (else
          (AI|BehaviorTree|FinishExecute false))))
    (:Is%20Not%20Valid
      (AI|BehaviorTree|FinishExecute false))))