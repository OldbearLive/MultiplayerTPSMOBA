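; Base weapon projectile actor that launches along its local X axis at ProjectileSpeed.
; On BeginPlay it waits a tick, sets the movement component's velocity, then attaches an optional tracer effect to the Arrow, parameterized by size and color.
; Box overlap only compares the other actor to the owner; the OnOverlap, collision-disable and delayed-destroy chain is disconnected, so it never runs.
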(event OnComponentBeginOverlap(BoxComponent)
  (params (OverlappedComponent :type Primitive%20Component%20Object%20Reference) (OtherActor :type Actor%20Object%20Reference) (OtherComp :type Primitive%20Component%20Object%20Reference) (OtherBodyIndex :type Integer) (bFromSweep :type Boolean) (SweepResult :type Hit%20Result%20Structure%20%28by%20ref%29))
  (if (== OtherActor (Components|GetOwner))
    _))

(event EventBeginPlay
  (Utilities|FlowControl|Delay 0.0)
  (Game|Components|ProjectileMovement|SetVelocityinLocalSpace (Variables|Default|GetProjectileMovementComponent) (Math|Vector|MakeVector (Variables|Default|GetProjectileSpeed) 0.0 0.0))
  (Utilities|IsValid (Variables|Default|GetTracer_TailSystem)
    (:Is%20Valid
      (bind _returnvalue (Niagara|SpawnSystemAttached (Variables|Default|GetTracer_TailSystem) (Variables|Default|GetArrow) "None" "0, 0, 0" "0, 0, 0" "KeepRelativeOffset" true))
      (bind _output_get (Variables|Default|SetTracerTailComponent _returnvalue))
      (Niagara|SetNiagaraVariable(Float) _output_get "SizeMultiplier" (Variables|Default|GetSize))
      (Niagara|SetNiagaraVariable(LinearColor) _output_get "Color" (Variables|Default|GetIn%20Value)))))

(event Collision|EventActorBeginOverlap
  (params (OtherActor :type Actor%20Object%20Reference)))

(event EventTick
  (params (DeltaSeconds :type Float%20%28single-precision%29)))

(fn ConstructionScript)