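; Base enemy Blueprint providing targeting support and shield hit feedback.
; Lock-on toggles a marker sphere, a facing event updates a Motion Warping target, and a pawn line trace to the target actor stores player distance and flags the enemy targetable.
; Shield hits apply a dynamic overlay material to the mesh, with a timeline fading its Visibility forward and back before clearing it.
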(event Custom|Shield%20HitEvent
  ;[1 1 1] Shield HitLogic
  (Utilities|IsValid (Rendering|Material|GetOverlayMaterial (Variables|Character|GetMesh) :!class /Script/Engine.MeshComponent)
    (:Is%20Valid
      (bind (_direction _newtrack_0) (Timeline|Timeline PlayFromStart)
        (:Update
          (Rendering|Material|SetScalarParameterValue (Variables|Default|GetShieldMaterialDynamicMaterial) "Visibility" _newtrack_0 :!class /Script/Engine.MaterialInstanceDynamic))
        (:Finished
          (switch Utilities|FlowControl|Switch|SwitchonETimelineDirection _direction
            (:Forward
              (CallFunction|ReverseShield))
            (:Backward
              (Rendering|Material|SetOverlayMaterial (Variables|Character|GetMesh) 0 :!class /Script/Engine.MeshComponent))))))
    (:Is%20Not%20Valid
      (bind _returnvalue (Rendering|Material|CreateDynamicMaterialInstance (Variables|Default|GetShield%20Material) "None" "None" :!class /Script/Engine.KismetMaterialLibrary))
      (Variables|Default|SetShieldMaterialDynamicMaterial _returnvalue)
      (Rendering|Material|SetOverlayMaterial (Variables|Character|GetMesh) (Variables|Default|GetShieldMaterialDynamicMaterial) :!class /Script/Engine.MeshComponent)
      (Timeline|Timeline PlayFromStart))))

(event Custom|reverseShield
  ;[1 1 1] Shield HitLogic
  (bind (_direction _newtrack_0) (Timeline|Timeline Reverse)
    (:Update
      (Rendering|Material|SetScalarParameterValue (Variables|Default|GetShieldMaterialDynamicMaterial) "Visibility" _newtrack_0 :!class /Script/Engine.MaterialInstanceDynamic))
    (:Finished
      (switch Utilities|FlowControl|Switch|SwitchonETimelineDirection _direction
        (:Forward
          (CallFunction|ReverseShield))
        (:Backward
          (Rendering|Material|SetOverlayMaterial (Variables|Character|GetMesh) 0 :!class /Script/Engine.MeshComponent))))))

(event EventBeginPlay)

(event Collision|EventActorBeginOverlap
  (params (OtherActor :type Actor%20Object%20Reference)))

(event EventTick
  (params (DeltaSeconds :type Float%20%28single-precision%29)))

(event EventUpdateFacingTarget
  (params (Target :type Vector%20%28by%20ref%29 :default "0, 0, 0"))
  (Class|MotionWarpingComponent|AddorUpdateWarpTargetfromLocation (Variables|Default|GetMotionWarping) "FacingTarget" Target))

(event EventLockon
  (bind _lockonsphere (Variables|Default|GetLockOnSphere))
  (Utilities|FlowControl|FlipFlop
    (:A
      (Rendering|SetVisibility _lockonsphere true false))
    (:B
      (Rendering|SetVisibility _lockonsphere false false))))

(fn ConstructionScript)

(fn DistancetoPlayer
  (Utilities|IsValid (Variables|Default|GetTargetActor)
    (:Is%20Valid
      (bind _outhit (Collision|LineTraceForObjects (Transformation|GetActorLocation) (Transformation|GetActorLocation (Variables|Default|GetTargetActor)) (Utilities|Array|MakeArray "ObjectTypeQuery3") false (Utilities|Array|MakeArray self) "ForDuration" true "(R=1.000000,G=0.000000,B=0.000000,A=1.000000)" "(R=0.000000,G=1.000000,B=0.000000,A=1.000000)" 1.0))
      (Variables|Default|SetPlayerToEnemyDistance (.Distance (Collision|BreakHitResult _outhit)))
      (Variables|Default|SetCanBeTargeted? true))))