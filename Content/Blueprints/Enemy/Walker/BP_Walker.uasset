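; BP_Walker is the Walker enemy Blueprint, supplying the creature's attack montages, combat socket locations and hit reactions.
; On BeginPlay it sets up a screen-space multiplayer stats bar widget with itself as the widget controller.
; Combat socket location follows the playing montage, choosing the left or right foot socket for the matching foot attack.
; Other getters return a random hit-react montage and the status widget's world location.
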(event EventBeginPlay
  (bind _remotestatsbar (Variables|Default|GetRemoteStatsBar))
  (|CallParentFunction)
  (bind _aswbp_multiplayer_stats (Utilities|Casting|CastToWBP_MultiplayerStats (UserInterface|GetWidget (Variables|Default|GetRemoteStatsBar))))
  (Variables|Default|SetAs%20WBP%20Multiplayer%20Stats _aswbp_multiplayer_stats)
  (UserInterface|SetWidget _remotestatsbar (Variables|Default|GetAs%20WBP%20Multiplayer%20Stats))
  (Class|WidgetComponent|SetWidgetSpace _remotestatsbar "Screen")
  (Class|CombatUserWidget|SetWidgetController (Variables|Default|GetAs%20WBP%20Multiplayer%20Stats) self))

(event Collision|EventActorBeginOverlap
  (params (OtherActor :type Actor%20Object%20Reference))
  (|CallParentFunction OtherActor) ; This node is disabled and will not be called.\nDrag off pins to build functionality.
)

(event EventTick
  (params (DeltaSeconds :type Float%20%28single-precision%29))
  (|CallParentFunction DeltaSeconds) ; This node is disabled and will not be called.\nDrag off pins to build functionality.
)

(fn ConstructionScript
  (|CallParentFunction))

(fn GetStatusWidgetLocation
  (return (Transformation|GetWorldLocation (Variables|Default|GetStatusWidgetTransform))))

(fn GetHitReactMontage
  (return (.OutItem (Utilities|Array|Random (Variables|Default|GetHitReactMontage)))))

(fn GetCombatSocketLocation
  (bind _returnvalue (Animation|GetCurrentMontage :!class /Script/Engine.Character))
  (Utilities|IsValid _returnvalue
    (:Is%20Valid
      (if (== _returnvalue "/Game/ImportedContent/Walker_2/Waker_2_L_Foot_Attack_Montage.Waker_2_L_Foot_Attack_Montage")
        (return (Transformation|GetSocketLocation (Variables|Character|GetMesh) "Foot_CombatSocket_L"))
        (elif (== _returnvalue "/Game/ImportedContent/Walker_2/Waker_2_R_Foot_Attack_Montage.Waker_2_R_Foot_Attack_Montage")
          (return (Transformation|GetSocketLocation (Variables|Character|GetMesh) "Foot_CombatSocket_R")))))))

(fn GetAttackMontages
  (return (Variables|Default|GetAttackMontages)))