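; Player controller for the multiplayer menu and lobby, handling menu input, lobby and loading screen widgets, and leaving a session back to MainMenu.
; InitialSetup loads or creates the local profile save, then sends it to the server, which stores it and has BP_CombatMenuGameMode update the lobby.
; Events pass player names and level selection into the lobby widget, which, like the loading screen, is created on first show and reused.
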(event Custom|UpdateLevelSelection
  (params (LevelRowName :type Name))
  (bind _wb_lobbymenu (Variables|Default|GetWB_LobbyMenu)
    (:then
      (Default|UpdateLevelSelection _wb_lobbymenu LevelRowName))
    (:else)))

(event Custom|Client_CreateLobbyMenuEvent
  (CallFunction|UIShowLobbyMenu))

(event Custom|UpdatePlayerNames
  (params (NewParam :type Array%20of%20S%20Player%20Profile%20Structures))
  (bind _wb_lobbymenu (Variables|Default|GetWB_LobbyMenu))
  (Utilities|IsValid _wb_lobbymenu
    (:Is%20Valid
      (Default|ClearPlayerNames _wb_lobbymenu)
      (Default|UpdatePlayerNames _wb_lobbymenu NewParam))))

(event Custom|EndClientSession
  (|DestroySession self
    (:then
      (Game|OpenLevel(byName) "MainMenu"))))

(event Custom|Client_CreateLoadScreen
  (CallFunction|UIShowLoadingScreen))

(event Custom|Server_UpdateLobby
  (params (PlayerInfo :type S%20Player%20Profile%20Structure))
  (Variables|Default|SetPlayer%20Profile%20Struct PlayerInfo)
  (bind _asbp_combat_menu_game_mode (Utilities|Casting|CastToBP_CombatMenuGameMode (Game|GetGameMode)))
  (Default|UpdateLobby _asbp_combat_menu_game_mode true true))

(event Custom|InitialSetup
  (CallFunction|LoadSavedProfile)
  (CallFunction|ServerUpdateLobby (Variables|Default|GetPlayer%20Profile%20Struct)))

(event EventBeginPlay
  (if (Pawn|IsLocalController)
    (Variables|Default|SetbShowMouseCursor true)
    (Input|SetInputModeUIOnly self 0 "DoNotLock" false)))

(fn ConstructionScript)

(fn UIShowLobbyMenu
  (Utilities|IsValid (Variables|Default|GetWB_LobbyMenu)
    (:Is%20Valid
      _)
    (:Is%20Not%20Valid
      (bind _returnvalue (UserInterface|CreateWidget "/Game/Blueprints/Multiplayer/UI/W_LobbyMenu.W_LobbyMenu_C" self))
      (Variables|Default|SetWB_LobbyMenu _returnvalue)))
  (UserInterface|Viewport|AddtoViewport (Variables|Default|GetWB_LobbyMenu) 0)
  (return))

(fn LoadSavedProfile
  (bind _returnvalue (SaveGame|DoesSaveGameExist (LocalVariables|GetLocal_SlotName)))
  (if _returnvalue
    _
    (else
      (bind _returnvalue_2 (SaveGame|CreateSaveGameObject "/Game/Blueprints/Multiplayer/SavedData/SG_PlayerProfile.SG_PlayerProfile_C"))
      (SaveGame|SaveGametoSlot _returnvalue_2 (LocalVariables|GetLocal_SlotName))))
  (bind _returnvalue_3 (SaveGame|LoadGamefromSlot (LocalVariables|GetLocal_SlotName)))
  (bind _assg_player_profile (Utilities|Casting|CastToSG_PlayerProfile _returnvalue_3))
  (Variables|Default|SetPlayer%20Profile%20Struct (Variables|/Game/Blueprints/Multiplayer/SavedData/SG_PlayerProfile.SG_PlayerProfile_C|GetPlayerProfileStruct _assg_player_profile))
  (return))

(fn UIHideLobbyMenu
  (Utilities|IsValid (Variables|Default|GetWB_LobbyMenu)
    (:Is%20Valid
      (Widget|RemovefromParent (Variables|Default|GetWB_LobbyMenu))
      (return))))

(fn UIShowLoadingScreen
  (Utilities|IsValid (Variables|Default|GetWB_LoadScreen)
    (:Is%20Valid
      _)
    (:Is%20Not%20Valid
      (bind _returnvalue (UserInterface|CreateWidget "/Game/Blueprints/Multiplayer/UI/W_LoadingScreen.W_LoadingScreen_C" self))
      (Variables|Default|SetWB_LoadScreen _returnvalue)))
  (UserInterface|Viewport|AddtoViewport (Variables|Default|GetWB_LoadScreen) 0)
  (return))

(fn UIHideLoadScreen
  (Utilities|IsValid (Variables|Default|GetWB_LoadScreen)
    (:Is%20Valid
      (Widget|RemovefromParent (Variables|Default|GetWB_LoadScreen))
      (return))))