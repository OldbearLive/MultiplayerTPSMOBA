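; Game mode for the multiplayer combat menu that manages connected players in the lobby level.
; New players in the Lobby level have their BP_MenuController registered, get a client lobby menu and run initial setup.
; UpdateLobby rebuilds the profile list from all controllers and pushes player names or the selected level name to each one.
; Logout removes the controller and refreshes everyone's player list.
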(event Custom|UpdateLobby
  (params (UpdatePlayers :type Boolean) (UpdateLevel :type Boolean))
  (if UpdatePlayers
    (Utilities|Array|Clear (Variables|Default|GetAllPlayerProfiles))
    (for _array_element (Variables|Default|GetAllConnectedPlayers)
      (Utilities|Array|Add (Variables|Default|GetAllPlayerProfiles) (Variables|/Game/Blueprints/Multiplayer/BP_MenuController.BP_MenuController_C|GetPlayer%20Profile%20Struct _array_element))))
  (for _array_element_2 (Variables|Default|GetAllConnectedPlayers)
    (if UpdatePlayers
      (Default|UpdatePlayerNames _array_element_2 (Variables|Default|GetAllPlayerProfiles)))
    (if UpdateLevel
      (Default|UpdateLevelSelection _array_element_2 (Variables|Default|GetSelectedLevelName)))))

(event EventBeginPlay)

(event EventTick
  (params (DeltaSeconds :type Float%20%28single-precision%29)))

(event EventHandleStartingNewPlayer
  (params (NewPlayer :type Player%20Controller%20Object%20Reference))
  (bind _returnvalue (Game|GetCurrentLevelName true))
  (switch string _returnvalue
    (:Lobby
      (bind _asbp_menu_controller (Utilities|Casting|CastToBP_MenuController NewPlayer))
      (Utilities|Array|Add (Variables|Default|GetAllConnectedPlayers) _asbp_menu_controller)
      (Default|ClientCreateLobbyMenuEvent _asbp_menu_controller)
      (Default|InitialSetup _asbp_menu_controller))))

(event EventOnLogout
  (params (ExitingController :type Controller%20Object%20Reference))
  (bind _asbp_menu_controller (Utilities|Casting|CastToBP_MenuController ExitingController))
  (Utilities|Array|RemoveItem (Variables|Default|GetAllConnectedPlayers) _asbp_menu_controller)
  (CallFunction|UpdateLobby true false))

(fn ConstructionScript)