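; Jetpack Blueprint that drives Niagara exhaust effects for a main thruster and four side thrusters, with activate, deactivate and dash events.
; DashAnimation plays a timeline that sets thruster size and velocity through FInterpTo with constant endpoints, then DashReset reverses it.
; Reverse completion clears the Dash flag on only one side thruster.
; BeginPlay registers the Blueprint as Niagara callback handler, and ParticleData prints received particle sizes.
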(event Custom|DeactivateJet
  (for _array_element (Variables|Default|GetJet_SideThrusters)
    (Components|Activation|Deactivate _array_element)))

(event Custom|DashReset
  (for _array_element (Variables|Default|GetJet_SideThrusters)
    (Effects|Components|ParticleSystem|SetBoolParameter _array_element "Dash" true))
  (bind _direction (Timeline|DashTimeline ReverseFromEnd)
    (:Update
      (if (Utilities|Enum|Equal(Enum) _direction "Forward")
        (Effects|Components|ParticleSystem|SetFloatParameter (Variables|Default|GetNiagara6) "SizeScale" (Math|Interpolation|FInterpTo 5.0 2e+01 (Utilities|Time|GetWorldDeltaSeconds) 5e+02))
        (Effects|Components|ParticleSystem|SetFloatParameter (Variables|Default|GetNiagara6) "Velocity Speed" (Math|Interpolation|FInterpTo 2e+01 5e+01 (Utilities|Time|GetWorldDeltaSeconds) 1e+02))
        (for _array_element_2 (Variables|Default|GetJet_SideThrusters)
          (Effects|Components|ParticleSystem|SetFloatParameter _array_element_2 "SizeScale" (Math|Interpolation|FInterpTo 1.0 1e+01 (Utilities|Time|GetWorldDeltaSeconds) 5e+02))
          (Effects|Components|ParticleSystem|SetFloatParameter _array_element_2 "Velocity Speed" (Math|Interpolation|FInterpTo 3.0 1e+01 (Utilities|Time|GetWorldDeltaSeconds) 2e+02)))
        (else
          (Effects|Components|ParticleSystem|SetFloatParameter (Variables|Default|GetNiagara6) "SizeScale" (Math|Interpolation|FInterpTo 2e+01 5.0 (Utilities|Time|GetWorldDeltaSeconds) 5e+02))
          (Effects|Components|ParticleSystem|SetFloatParameter (Variables|Default|GetNiagara6) "Velocity Speed" (Math|Interpolation|FInterpTo 5e+01 2e+01 (Utilities|Time|GetWorldDeltaSeconds) 1e+02))
          (for _array_element_3 (Variables|Default|GetJet_SideThrusters)
            (Effects|Components|ParticleSystem|SetFloatParameter _array_element_3 "SizeScale" (Math|Interpolation|FInterpTo 1e+01 1.0 (Utilities|Time|GetWorldDeltaSeconds) 5e+02))
            (Effects|Components|ParticleSystem|SetFloatParameter _array_element_3 "Velocity Speed" (Math|Interpolation|FInterpTo 1e+01 3.0 (Utilities|Time|GetWorldDeltaSeconds) 2e+02))))))
    (:Finished
      (if (Utilities|Enum|Equal(Enum) _direction "Forward")
        (CallFunction|DashReset)
        (else
          (Effects|Components|ParticleSystem|SetBoolParameter (Variables|Default|GetNiagara) "Dash" false))))))

(event Custom|ActivateJet
  (for _array_element (Variables|Default|GetJet_SideThrusters)
    (Components|Activation|Activate _array_element true)))

(event Custom|DashAnimation
  (for _array_element (Variables|Default|GetJet_SideThrusters)
    (Effects|Components|ParticleSystem|SetBoolParameter _array_element "Dash" true))
  (bind _direction (Timeline|DashTimeline PlayFromStart)
    (:Update
      (if (Utilities|Enum|Equal(Enum) _direction "Forward")
        (Effects|Components|ParticleSystem|SetFloatParameter (Variables|Default|GetNiagara6) "SizeScale" (Math|Interpolation|FInterpTo 5.0 2e+01 (Utilities|Time|GetWorldDeltaSeconds) 5e+02))
        (Effects|Components|ParticleSystem|SetFloatParameter (Variables|Default|GetNiagara6) "Velocity Speed" (Math|Interpolation|FInterpTo 2e+01 5e+01 (Utilities|Time|GetWorldDeltaSeconds) 1e+02))
        (for _array_element_2 (Variables|Default|GetJet_SideThrusters)
          (Effects|Components|ParticleSystem|SetFloatParameter _array_element_2 "SizeScale" (Math|Interpolation|FInterpTo 1.0 1e+01 (Utilities|Time|GetWorldDeltaSeconds) 5e+02))
          (Effects|Components|ParticleSystem|SetFloatParameter _array_element_2 "Velocity Speed" (Math|Interpolation|FInterpTo 3.0 1e+01 (Utilities|Time|GetWorldDeltaSeconds) 2e+02)))
        (else
          (Effects|Components|ParticleSystem|SetFloatParameter (Variables|Default|GetNiagara6) "SizeScale" (Math|Interpolation|FInterpTo 2e+01 5.0 (Utilities|Time|GetWorldDeltaSeconds) 5e+02))
          (Effects|Components|ParticleSystem|SetFloatParameter (Variables|Default|GetNiagara6) "Velocity Speed" (Math|Interpolation|FInterpTo 5e+01 2e+01 (Utilities|Time|GetWorldDeltaSeconds) 1e+02))
          (for _array_element_3 (Variables|Default|GetJet_SideThrusters)
            (Effects|Components|ParticleSystem|SetFloatParameter _array_element_3 "SizeScale" (Math|Interpolation|FInterpTo 1e+01 1.0 (Utilities|Time|GetWorldDeltaSeconds) 5e+02))
            (Effects|Components|ParticleSystem|SetFloatParameter _array_element_3 "Velocity Speed" (Math|Interpolation|FInterpTo 1e+01 3.0 (Utilities|Time|GetWorldDeltaSeconds) 2e+02))))))
    (:Finished
      (if (Utilities|Enum|Equal(Enum) _direction "Forward")
        (CallFunction|DashReset)
        (else
          (Effects|Components|ParticleSystem|SetBoolParameter (Variables|Default|GetNiagara) "Dash" false))))))

(event EventBeginPlay
  (for _array_element (Variables|Default|GetJet_SideThrusters)
    (Class|NiagaraComponent|SetVariableObject _array_element "User.BP_CallbackHandler" self)))

(event EventParticleData
  (params (Data :type Array%20of%20Basic%20Particle%20Data%20Structures) (NiagaraSystem :type Niagara%20System%20Object%20Reference) (SimulationPositionOffset :type Vector%20%28by%20ref%29 :default "0, 0, 0"))
  (for _array_element Data
    (bind _output_get (Variables|Default|SetCurrentSystemVelocity (.Size (Utilities|Struct|BreakBasicParticleData _array_element))))
    (Development|PrintString (Utilities|String|ToString(Float) _output_get))))

(fn ConstructionScript
  (Variables|Default|SetJet_L_FX (Utilities|Array|MakeArray 0 (Variables|Default|GetNiagara) (Variables|Default|GetNiagara2)))
  (Variables|Default|SetJet_R_FX (Utilities|Array|MakeArray 0 (Variables|Default|GetNiagara5) (Variables|Default|GetNiagara3)))
  (Variables|Default|SetJet_SideThrusters (Utilities|Array|MakeArray (Variables|Default|GetNiagara) (Variables|Default|GetNiagara2) (Variables|Default|GetNiagara5) (Variables|Default|GetNiagara3))))