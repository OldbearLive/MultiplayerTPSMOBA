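; Base actor component that equips a weapon animation layer on its owning Character.
; On BeginPlay it caches the mesh and movement component, then notifies the owner through an interface message.
; EquipAnimLayer zeroes max acceleration during the equip montage, then spawns and socket-attaches the weapon, links the anim class layer and resets acceleration to a hard-coded default.
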(event EventBeginPlay
  ;[1 1 1 1 30] BeginPlay Call Interface event on Main Character. Sends information about self and the animlayer it's sending. (ended up not using the anim layer information in my case)
  (bind _output_get (Variables|Default|SetSkeletalMesh (Actor|GetComponentbyClass (Components|GetOwner) "/Script/Engine.SkeletalMeshComponent")))
  (Utilities|IsValid _output_get
    (:Is%20Valid
      (bind _ascharacter (Utilities|Casting|CastToCharacter (Components|GetOwner)))
      (bind _output_get_2 (Variables|Default|Set%20Character _ascharacter))
      (bind _ascharacter_movement_component (Utilities|Casting|CastToCharacterMovementComponent (Pawn|GetMovementComponent _output_get_2)))
      (Variables|Default|SetCharacter%20Movement%20Component _ascharacter_movement_component)
      (Class|BPILinkAnimLayers|EquipComponent(Message) (Components|GetOwner) (Variables|Default|GetAnimLayer) (Variables|Default|GetAnim%20Layer%20Component)))))

(event EventEquipAnimLayer
  (params (AnimLayer :type Anim%20Instance%20Class%20Reference))
  ;[1 1 1 1 30] Called from the Player. Uses the same Interface, here this acts as a listener and links the abstract anim layer instance.
  (Utilities|IsValid (Variables|Default|GetSkeletalMesh)
    (:Is%20Valid
      (bind _returnvalue (Animation|PlayAnimMontage (Variables|Default|Get%20Character) (Variables|Default|GetEquipMontage) 1.0 "None"))
      (Variables|/Script/Engine.CharacterMovementComponent|SetMaxAcceleration (Variables|Default|GetCharacter%20Movement%20Component) 0.0)
      (Utilities|FlowControl|Delay (- _returnvalue 0.3))
      (if (Utilities|IsValidClass (Variables|Default|GetWeaponActor))
        (bind _returnvalue_2 (Game|SpawnActorfromClass (Variables|Default|GetWeaponActor) (Math|Transform|MakeTransform "0, 0, 0" "0, 0, 0" "1.000000,1.000000,1.000000") "Undefined" 0 0))
        (Transformation|AttachComponentToComponent _returnvalue_2 (Variables|Default|GetSkeletalMesh) (Variables|Default|GetAttachSocketName) "SnapToTarget" "SnapToTarget" "SnapToTarget" true))
      (Components|SkeletalMesh|AnimationBlueprintLinking|LinkAnimClassLayers (Variables|Default|GetSkeletalMesh) AnimLayer)
      (Variables|/Script/Engine.CharacterMovementComponent|SetMaxAcceleration (Variables|Default|GetCharacter%20Movement%20Component) 2048.0))))

(fn GetDefaultMaxAcceleration
  (return 0.0))