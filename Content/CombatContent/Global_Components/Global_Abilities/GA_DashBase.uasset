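; Base dash gameplay ability that locks rotation, applies a dashing state effect and plays a montage.
; The montage's DashReady event spawns Niagara FX and applies constant-force root motion.
; After the montage, it either activates the sprint ability or sends a dash-release event and ends, based on input release.
; When locked on, it orients rotation to movement during the dash, restoring strafing on end.
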(event Custom|StartSprinting
  (bind _returnvalue (Ability|GetActorInfo))
  (bind _dashfx (Variables|Default|GetDashFX))
  (bind (_owneractor _avataractor _playercontroller _abilitysystemcomponent) (Utilities|Struct|BreakGameplayAbilityActorInfo _returnvalue))
  (if (Components|Activation|IsActive _dashfx)
    (Components|Activation|Deactivate _dashfx))
  ;[0 0 0] Sprint Function
  (bind _ascharacter (Utilities|Casting|CastToCharacter _avataractor))
  (Rendering|SetVisibility (Variables|/Script/Engine.Character|GetCapsuleComponent _ascharacter) true true)
  (bind _returnvalue_2 (Abilities|TryActivateAbilitybyClass _abilitysystemcomponent (Variables|Default|GetSprintAbilitytoActivate) true))
  (Development|PrintString (Utilities|String|ToString(Boolean) _returnvalue_2)))

(event Custom|ResetOrientRotaion
  (bind _returnvalue (Ability|GetActorInfo))
  (bind (_owneractor _avataractor _playercontroller _abilitysystemcomponent _skeletalmeshcomponent _animinstance _movementcomponent) (Utilities|Struct|BreakGameplayAbilityActorInfo _returnvalue))
  (if (Class|GSCBlueprintFunctionLibrary|HasAnyMatchingGameplayTag _avataractor "(GameplayTags=((TagName=\"Player.Loose.isLockON\")))")
    (bind _ascharacter_movement_component (Utilities|Casting|CastToCharacterMovementComponent _movementcomponent))
    (Variables|/Script/Engine.CharacterMovementComponent|SetbOrientRotationToMovement _ascharacter_movement_component false)))

(event Ability|EventActivateAbility
  (bind _returnvalue (Ability|GetActorInfo))
  (bind _returnvalue_2 (Ability|GetActorInfo))
  (bind _movement_direction (Variables|Default|GetMovement_Direction))
  (bind (_owneractor _avataractor _playercontroller _abilitysystemcomponent _skeletalmeshcomponent _animinstance _movementcomponent) (Utilities|Struct|BreakGameplayAbilityActorInfo _returnvalue))
  (bind _avataractor_2 (Utilities|Struct|BreakGameplayAbilityActorInfo _returnvalue_2))
  (bind _returnvalue_3 (Ability|CommitAbility))
  (if _returnvalue_3
    (bind _ascharacter_movement_component (Utilities|Casting|CastToCharacterMovementComponent _movementcomponent))
    (bind _output_get (Variables|Default|SetAs%20Character%20Movement%20Component _ascharacter_movement_component))
    (Variables|/Script/Engine.CharacterMovementComponent|SetRotationRate _output_get "0, 0, 0")
    (if (Class|GSCBlueprintFunctionLibrary|HasAnyMatchingGameplayTag _avataractor "(GameplayTags=((TagName=\"Player.Loose.isLockON\")))")
      ;[0 0 0] If was Strafe Movement, Bind to reset orient rotation to movement function
      (bind _ascharacter_movement_component_2 (Utilities|Casting|CastToCharacterMovementComponent (.MovementComponent (Utilities|Struct|BreakGameplayAbilityActorInfo (Ability|GetActorInfo)))))
      (Variables|/Script/Engine.CharacterMovementComponent|SetbOrientRotationToMovement _ascharacter_movement_component_2 true)
      (EventDispatchers|BindEventtoOnAbilityEnded (EventDispatchers|CreateEvent :!event Custom|ResetOrientRotaion)))
    (Ability|ApplyGameplayEffectToOwner (Variables|Default|GetStateTagEffect))
    (|PlayMontageandWaitforEvent "None" (Variables|Default|GetDashMontage) "(GameplayTags=((TagName=\"Player.Event.DashReady\")))" 1.0 "None" false 0.0
      (:OnCompleted
        (bind _timeheld (Ability|Tasks|WaitInputRelease true :!label _label)
          (:then
            (if (== _timeheld 0.0)
              (CallFunction|StartSprinting)
              (else
                (Ability|SendGameplayEventtoActor _avataractor_2 "(TagName=\"Player.Input.Dash.Release\")")
                (Ability|EndAbility))))
          (:OnRelease
            (Ability|SendGameplayEventtoActor _avataractor_2 "(TagName=\"Player.Input.Dash.Release\")")
            (Ability|EndAbility))))
      (:OnBlendOut
        (goto _label))
      (:OnInterrupted
        (Ability|EndAbility :!label _label_2))
      (:OnCancelled
        (goto _label_2))
      (:EventReceived
        (bind _asbp_base_character (Utilities|Casting|CastToBP_BaseCharacter (.AvatarActor (Utilities|Struct|BreakGameplayAbilityActorInfo (Ability|GetActorInfo)))))
        (bind _returnvalue_4 (Niagara|SpawnSystemAttached (Variables|Default|GetDashFXSystem) (Variables|/Game/CombatContent/Characters/BP_BaseCharacter.BP_BaseCharacter_C|GetRootScene _asbp_base_character) "None" (Transformation|GetActorLocation _asbp_base_character) (Math|Rotator|MakeRotator 0.0 0.0 (.yaw (Math|Rotator|MakeRotfromX (Transformation|GetActorForwardVector _asbp_base_character)))) "KeepWorldPosition" true))
        (Variables|Default|SetDashFX _returnvalue_4)
        (Ability|Tasks|ApplyRootMotionConstantForce "None" _movement_direction (Variables|Default|GetMovementMagnitude) 0.0 false 0 "SetVelocity" (* _movement_direction 3e+03)
          (:then
            (bind _ascharacter (Utilities|Casting|CastToCharacter (.AvatarActor (Utilities|Struct|BreakGameplayAbilityActorInfo (Ability|GetActorInfo)))))
            (Rendering|SetVisibility (Variables|/Script/Engine.Character|GetCapsuleComponent _ascharacter) true true)))))
    (else
      (Ability|CancelAbility))))

(event Ability|EventOnEndAbility
  (params (bWasCancelled :type Boolean))
  (bind _returnvalue (Ability|GetActorInfo))
  (bind _dashfx (Variables|Default|GetDashFX))
  (bind _avataractor (Utilities|Struct|BreakGameplayAbilityActorInfo _returnvalue))
  (bind _rotationrate (Class|BPIGetPlayerInfo|GetWalkSpeedandMaxWalkSpeed(Message) _avataractor))
  (Variables|/Script/Engine.CharacterMovementComponent|SetRotationRate (Variables|Default|GetAs%20Character%20Movement%20Component) _rotationrate)
  (bind _ascharacter (Utilities|Casting|CastToCharacter _avataractor))
  (Rendering|SetVisibility (Variables|/Script/Engine.Character|GetCapsuleComponent _ascharacter) true true)
  (Ability|RemoveGameplayEffectFromOwnerWithGrantedTags "(GameplayTags=((TagName=\"Player.State.IsDashing\")))")
  (Ability|SendGameplayEventtoActor _avataractor "(TagName=\"Player.Input.Dash.Release\")")
  (Utilities|IsValid _dashfx
    (:Is%20Valid
      (Components|Activation|Deactivate _dashfx))))

(fn GetWalkSpeedandMaxWalkSpeed
  (return 0.0 0.0 "0, 0, 0"))

(fn GetBaseWeapon
  (return 0))