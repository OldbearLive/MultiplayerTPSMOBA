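; Base gameplay ability for AI melee attacks, which commits only with a valid target and plays an attack montage.
; A Block event applies a probability effect and plays a deflection montage, where an optional CanAttack event triggers a wake-up attack that can itself be deflected.
; Montage-and-wait-for-event tasks drive each stage, with the current one cached for manual termination.
; A Hit branch exists, but the attack montage listens only for Block.
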(event Custom|WakeUpDelegate
  (if (Variables|Default|GetShould%20Wakeup%20Attack?)
    (Utilities|IsValid (Variables|Default|GetAsync%20Task)
      (:Is%20Valid
        (GameplayTasks|EndTask (Variables|Default|GetAsync%20Task))
        (Variables|Default|SetAsync%20Task 0)
        (bind _asynctaskproxy (|PlayMontageandWaitforEvent "None" (Variables|Default|GetWakeUpAttackMontage) (select (Variables|Default|GetShould%20Block%20Wakeup?) "(GameplayTags=((TagName=\"Event.AI.Received.Block\")))" "") 1.0 "None" false 1.0)
          (:then
            (Variables|Default|SetAsync%20Task _asynctaskproxy))
          (:OnCompleted
            (Ability|EndAbility :!label _label))
          (:OnBlendOut
            (goto _label))
          (:OnInterrupted
            (goto _label))
          (:OnCancelled
            (goto _label))
          (:EventReceived
            (GameplayTasks|EndTask (Variables|Default|GetAsync%20Task))
            (Variables|Default|SetAsync%20Task 0)
            (|PlayMontageandWaitProxy "None" (Variables|Default|GetAttack_Deflection) 1.0 "None" false 1.0 0.0
              (:OnCompleted
                _)
              (:OnBlendOut
                _)
              (:OnInterrupted
                _)
              (:OnCancelled
                _))
            (Ability|EndAbility)))))
    (else
      (Ability|EndAbility))))

(event Custom|End%20and%20null%20task
  (Utilities|IsValid (Variables|Default|GetAsync%20Task)
    (:Is%20Valid
      (GameplayTasks|EndTask (Variables|Default|GetAsync%20Task))
      (Variables|Default|SetAsync%20Task 0))))

(event Ability|EventActivateAbility
  (bind _returnvalue (Ability|GetActorInfo))
  (bind _abilitysystemcomponent (Utilities|Struct|BreakGameplayAbilityActorInfo _returnvalue))
  (bind _asbp_ai_base (Utilities|Casting|CastToBP_AI_Base (.AvatarActor (Utilities|Struct|BreakGameplayAbilityActorInfo (Ability|GetActorInfo)))))
  (bind _output_get (Variables|Private|SetOwnerAI _asbp_ai_base))
  (Utilities|IsValid (Variables|/Game/CombatContent/Characters/AI/BP_AI_Base.BP_AI_Base_C|GetTargetActor _output_get)
    (:Is%20Valid
      (bind _returnvalue_2 (Ability|CommitAbility))
      (if _returnvalue_2
        (EventDispatchers|BindEventtoOnAbilityEnded (EventDispatchers|CreateEvent :!event Custom|End%20and%20null%20task))
        (bind (_asynctaskproxy _eventtag) (|PlayMontageandWaitforEvent "None" (Variables|Default|GetAttackMontage) "(GameplayTags=((TagName=\"Event.AI.Received.Block\"),(TagName=\"Event.AI.Received.Hit\")))" 1.0 "None" false 1.0)
          (:then
            (Variables|Default|SetAsync%20Task _asynctaskproxy))
          (:OnCompleted
            (Ability|EndAbility :!label _label))
          (:OnBlendOut
            (goto _label))
          (:OnInterrupted
            (goto _label))
          (:OnCancelled
            (goto _label))
          (:EventReceived
            (|SwitchGameplayTag _eventtag
              (:Event.AI.Received.Block
                (Variables|Private|SetHasBlocked? true)
                (GameplayEffects|ApplyGameplayEffectSpecToSelf _abilitysystemcomponent (GameplayEffects|MakeOutgoingSpec :self (Ability|GetAbilitySystemComponent (Variables|Private|GetOwnerAI)) :GameplayEffectClass (Variables|Default|GetProbabilityGameplayEffect)))
                (bind _asynctaskproxy_2 (|PlayMontageandWaitforEvent "None" (Variables|Default|GetAttack_Deflection) (select (Variables|Default|GetShould%20Wakeup%20Attack?) "(GameplayTags=((TagName=\"Event.AI.CanAttack\")))" "") 1.0 "None" false 1.0)
                  (:then
                    (Variables|Default|SetAsync%20Task _asynctaskproxy_2))
                  (:OnCompleted
                    (if (Variables|Private|GetIsWakingUpAttack?) :!label _label_2
                      (Utilities|IsValid (Variables|Default|GetAsync%20Task) :!label _label_3
                        (:Is%20Valid
                          (GameplayTasks|EndTask (Variables|Default|GetAsync%20Task))
                          (Variables|Default|SetAsync%20Task 0)
                          (bind _asynctaskproxy_3 (|PlayMontageandWaitforEvent "None" (Variables|Default|GetWakeUpAttackMontage) (select (Variables|Default|GetShould%20Block%20Wakeup?) "(GameplayTags=((TagName=\"Event.AI.Received.Block\")))" "") 1.0 "None" false 1.0)
                            (:then
                              (Variables|Default|SetAsync%20Task _asynctaskproxy_3))
                            (:OnCompleted
                              (Ability|EndAbility :!label _label_4))
                            (:OnBlendOut
                              (goto _label_4))
                            (:OnInterrupted
                              (goto _label_4))
                            (:OnCancelled
                              (goto _label_4))
                            (:EventReceived
                              (GameplayTasks|EndTask (Variables|Default|GetAsync%20Task))
                              (Variables|Default|SetAsync%20Task 0)
                              (|PlayMontageandWaitProxy "None" (Variables|Default|GetAttack_Deflection) 1.0 "None" false 1.0 0.0
                                (:OnCompleted
                                  _)
                                (:OnBlendOut
                                  _)
                                (:OnInterrupted
                                  _)
                                (:OnCancelled
                                  _))
                              (Ability|EndAbility)))))
                      (else
                        (Ability|EndAbility :!label _label_5))))
                  (:OnBlendOut
                    (goto _label_2))
                  (:OnInterrupted
                    (goto _label_5))
                  (:OnCancelled
                    (goto _label_5))
                  (:EventReceived
                    (Variables|Private|SetIsWakingUpAttack? true)
                    (Development|PrintString "Can Attack")
                    (goto _label_3))))
              (:Event.AI.Received.Hit
                (GameplayTasks|EndTask (Variables|Default|GetAsync%20Task))
                (Variables|Default|SetAsync%20Task 0)
                (GameplayEffects|ApplyGameplayEffectSpecToSelf _abilitysystemcomponent (GameplayEffects|MakeOutgoingSpec :self (Ability|GetAbilitySystemComponent (Variables|Private|GetOwnerAI)) :GameplayEffectClass (Variables|Default|GetProbabilityGameplayEffect)))
                (bind _payload (Ability|Tasks|WaitGameplayEvent "(TagName=\"Event.AI.CanAttack\")" 0)
                  (:then
                    (Ability|EndAbility))
                  (:EventReceived
                    (|SwitchGameplayTag (.EventTag (Utilities|Struct|BreakGameplayEventData _payload))
                      (:Default
                        (Ability|EndAbility))
                      (:Event.AI.CanAttack
                        (CallFunction|WakeUpDelegate)))))))))
        (else
          (Ability|CancelAbility :!label _label_6))))
    (:Is%20Not%20Valid
      (goto _label_6))))

(fn GetSkeletalMeshComponent
  (return 0))