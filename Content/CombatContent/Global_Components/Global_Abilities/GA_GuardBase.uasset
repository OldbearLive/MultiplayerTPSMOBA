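; GA_GuardBase is a base guard/block gameplay ability that puts the owner into a guarding state.
; On commit it applies a guarding tag effect, sets guard walk speed, enables orient-to-movement and optionally hides the weapon mesh, binding ability-end callbacks for cleanup.
; A guard montage listens for the blocked-attack event, which triggers a block montage that can outlive the ability.
; Either montage finishing or being interrupted ends the ability.
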(event Custom|Remove_GuardState
  (Ability|RemoveGameplayEffectFromOwnerWithGrantedTags "(GameplayTags=((TagName=\"Player.State.IsGuarding\")))"))

(event Custom|HideMeshEvent
  (Default|HideMesh (Variables|Default|GetBase%20Weapon%20Actor)))

(event Custom|UnHideMeshEvent
  (Default|UnHideMesh (Variables|Default|GetBase%20Weapon%20Actor)))

(event Custom|ResetMovementSpeed
  (bind _walkspeed (Class|BPIGetPlayerInfo|GetWalkSpeedandMaxWalkSpeed(Message) (.AvatarActor (Utilities|Struct|BreakGameplayAbilityActorInfo (Ability|GetActorInfo)))))
  (Variables|/Script/Engine.CharacterMovementComponent|SetMaxWalkSpeed (Variables|Default|GetAs%20Character%20Movement%20Component) _walkspeed))

(event Custom|ResetOrientRotation
  (Variables|/Script/Engine.CharacterMovementComponent|SetbOrientRotationToMovement (Variables|Default|GetAs%20Character%20Movement%20Component) false))

(event Ability|EventActivateAbility
  (bind _ascharacter_movement_component (Utilities|Casting|CastToCharacterMovementComponent (.MovementComponent (Utilities|Struct|BreakGameplayAbilityActorInfo (Ability|GetActorInfo)))))
  (Variables|Default|SetAs%20Character%20Movement%20Component _ascharacter_movement_component)
  (bind _returnvalue (Ability|CommitAbility))
  (if _returnvalue
    (Ability|ApplyGameplayEffectToOwner "/Game/CombatContent/Global_Components/Global_Abilities/AbilityEffects/GE_StateTag_Guarding.GE_StateTag_Guarding_C")
    (EventDispatchers|BindEventtoOnAbilityEnded (EventDispatchers|CreateEvent :!event Custom|Remove_GuardState))
    (Variables|/Script/Engine.CharacterMovementComponent|SetMaxWalkSpeed (Variables|Default|GetAs%20Character%20Movement%20Component) (Variables|Default|GetGuard_WalkSpeed))
    (EventDispatchers|BindEventtoOnAbilityEnded (EventDispatchers|CreateEvent :!event Custom|ResetMovementSpeed))
    (if (Variables|/Script/Engine.CharacterMovementComponent|GetbOrientRotationToMovement (Variables|Default|GetAs%20Character%20Movement%20Component))
      _
      (else
        (Variables|/Script/Engine.CharacterMovementComponent|SetbOrientRotationToMovement (Variables|Default|GetAs%20Character%20Movement%20Component) true)
        (EventDispatchers|BindEventtoOnAbilityEnded (EventDispatchers|CreateEvent :!event Custom|ResetOrientRotation))))
    (bind _baseweaponactor (Class|BPIGetPlayerInfo|GetBaseWeapon(Message) (Ability|GetAvatarActorfromActorInfo)))
    (Variables|Default|SetBase%20Weapon%20Actor _baseweaponactor)
    (if (Variables|Default|GetHideMesh?)
      (CallFunction|HideMeshEvent)
      (EventDispatchers|BindEventtoOnAbilityEnded (EventDispatchers|CreateEvent :!event Custom|UnHideMeshEvent)))
    (bind (_asynctaskproxy _eventtag) (|PlayMontageandWaitforEvent "None" (Variables|Default|GetGuardMontage) "(GameplayTags=((TagName=\"Event.Player.BlockedAttack\")))" 1.0 "None" true 1.0)
      (:then
        (if (Variables|Default|GetHasBlocked?)
          (GameplayTasks|EndTask _asynctaskproxy)))
      (:OnCompleted
        (Ability|EndAbility :!label _label))
      (:OnBlendOut
        (goto _label))
      (:OnInterrupted
        (goto _label))
      (:OnCancelled
        (goto _label))
      (:EventReceived
        (|SwitchGameplayTag _eventtag
          (:Event.Player.BlockedAttack
            (Variables|Default|SetHasBlocked? true)
            (|PlayMontageandWaitProxy "None" (Variables|Default|GetGuardBlockMontage) 1.0 "None" false 1.0 0.0
              (:OnCompleted
                _)
              (:OnBlendOut
                _)
              (:OnInterrupted
                _)
              (:OnCancelled
                _))
            (Ability|EndAbility)))))
    (else
      (Ability|CancelAbility))))

(event Ability|EventOnEndAbility
  (params (bWasCancelled :type Boolean)))

(fn GetWalkSpeedandMaxWalkSpeed
  (return 0.0 0.0 "0, 0, 0"))

(fn GetBaseWeapon
  (return 0))