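; Base weapon actor that provides swing trail, whoosh sound and mesh visibility controls, plus scaffolding for melee damage traces.
; BeginPlay attaches an inactive trail sized between the two trace sockets and an inactive sound, toggled by helper functions, with speed driving the sound.
; The server trace event stores the owning character and enables tick, but Tick is empty.
; The sphere-trace damage and knockback logic is disconnected, as are the multicast calls.
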(event Custom|Server_WeaponDamageTrace
  (params (Self%20Actor :type Actor%20Object%20Reference))
  ;[0 0.7188 0.1499] TraceReplication
  (CallFunction|WeaponTrace Self%20Actor))

(event Custom|MC_WeaponDamageTrace
  (params (Self%20Actor :type Actor%20Object%20Reference))
  ;[0 0.7188 0.1499] TraceReplication
)

(event Custom|WeaponTrace
  (params (Self%20Actor :type Actor%20Object%20Reference))
  ;[0 0 0] WeaponTraceEvent
  (bind _ascharacter (Utilities|Casting|CastToCharacter Self%20Actor))
  (Variables|Default|SetDamageOwner _ascharacter)
  (Variables|Weapon|Trace|Private|SetCanTrace? true)
  (Actor|Tick|SetActorTickEnabled true))

(event Custom|Server_DisableTrace
  ;[0 0.7188 0.1499] TraceReplication
)

(event Custom|MC_DisableTrace
  ;[0 0.7188 0.1499] TraceReplication
)

(event EventBeginPlay
  (bind _weapon_mesh (Variables|Default|GetWeapon_Mesh))
  ;[1 1 1] BeginPlayInitializations
  (Weapon|FX|AddAnimTrails)
  (bind _returnvalue (Audio|SpawnSoundAttached (Variables|Weapon|Sound|GetWhoosh_Sound) _weapon_mesh "None" (Transformation|GetWorldLocation _weapon_mesh) "0, 0, 0" "KeepWorldPosition" false 1.0 1.0 0.0 0 0 false))
  (bind _output_get (Variables|Default|SetSword_Sound _returnvalue))
  (Components|Activation|Deactivate _output_get))

(event EventTick
  (params (DeltaSeconds :type Float%20%28single-precision%29)))

(event EventHandleHitstop
  (params (HitStopDuration :type Float%20%28double-precision%29) (DamageOwnerActor :type Actor%20Object%20Reference)))

(event EventHandleInstantDamage
  (params (WeaponRawDamage :type Float%20%28double-precision%29) (DamageOwnerActor :type Actor%20Object%20Reference) (HitStopDuration :type Float%20%28double-precision%29) (HitWorldLocation :type Vector :default "0, 0, 0")))

(fn ConstructionScript)

(fn AddAnimTrails
  (bind _tracestartsocket (Variables|Weapon|Trace|GetTraceStartSocket))
  (bind _traceendsocket (Variables|Weapon|Trace|GetTraceEndSocket))
  (bind _weapon_mesh (Variables|Default|GetWeapon_Mesh))
  (bind _returnvalue (Transformation|GetSocketLocation _weapon_mesh _traceendsocket))
  (bind _returnvalue_2 (Transformation|GetSocketLocation _weapon_mesh _tracestartsocket))
  (bind _returnvalue_3 (- _returnvalue_2 _returnvalue))
  (bind _returnvalue_4 (Niagara|SpawnSystemAttached (Variables|Weapon|FX|GetWeaponTrailSystem) (Variables|Default|GetWeapon_Mesh) "None" (/ (+ _returnvalue_2 _returnvalue) 2.0) (Math|Rotator|MakeRotfromZ _returnvalue_3) "KeepWorldPosition" false))
  (Effects|Components|ParticleSystem|SetFloatParameter _returnvalue_4 "Trail_Width" (Math|Vector|VectorLength _returnvalue_3))
  (bind _output_get (Variables|Default|SetActiveTrailComponent _returnvalue_4))
  (Components|Activation|Deactivate _output_get)
  (return))

(fn ActivateSound
  (params (Speed :type Float%20%28single-precision%29))
  (bind _sword_sound (Variables|Default|GetSword_Sound))
  (Utilities|IsValid (Variables|Default|GetSword_Sound)
    (:Is%20Valid
      (Components|Activation|Activate _sword_sound false)
      (Audio|Parameter|SetFloatParameter _sword_sound "Speed" Speed :!class /Script/AudioExtensions.AudioParameterControllerInterface)
      (return))))

(fn ResetSound
  (bind _sword_sound (Variables|Default|GetSword_Sound))
  (Utilities|IsValid _sword_sound
    (:Is%20Valid
      (Components|Activation|Deactivate _sword_sound))))

(fn ResetTrail
  (bind _activetrailcomponent (Variables|Default|GetActiveTrailComponent))
  (Utilities|IsValid _activetrailcomponent
    (:Is%20Valid
      (Components|Activation|Deactivate _activetrailcomponent))))

(fn ActivateTrail
  (bind _activetrailcomponent (Variables|Default|GetActiveTrailComponent))
  (Utilities|IsValid _activetrailcomponent
    (:Is%20Valid
      (Components|Activation|Activate _activetrailcomponent true))))

(fn HideMesh
  (Rendering|SetVisibility (Variables|Default|GetWeapon_Mesh) false true))

(fn UnHideMesh
  (Rendering|SetVisibility (Variables|Default|GetWeapon_Mesh) true true))

(fn GetSkeletalMeshComponent
  (return (Variables|Default|GetWeapon_Mesh)))