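; Base player character for a GAS combat game, handling Enhanced Input movement, look and creation of the combat HUD on the local client.
; F cycles anim-layer components through server and multicast events, swapping each one's weapon-tag gameplay effect.
; GSCCore callbacks clamp Health and Armor and adjust them when their maximums change.
; Tick eases spring-arm length and offset based on dash and lock-on gameplay tags.
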(event Custom|MC_EquipAnimLayer
  (params (AnimLayerComponent :type Actor%20Component%20Object%20Reference) (AnimLayer :type Anim%20Instance%20Class%20Reference))
  ;[0 0 0 1 30] EquipAnimLayer_Replication
  (Class|BPILinkAnimLayers|EquipAnimLayer(Message) AnimLayerComponent AnimLayer))

(event Custom|Server_GetAnimLayerComponent
  ;[0 0 0] SwitchEquipment
  (CallFunction|MCGetAnimLayerComponent))

(event Custom|MC_GetAnimLayerComponent
  ;[0 0 0] SwitchEquipment
  (bind (_output_get _animlayer) (AnimationLayer|GetAnimLayerComponent))
  (CallFunction|ServerEquipAnimLayer _output_get _animlayer)
  (CallFunction|SwitchingEquipment)
  (Development|PrintString "SwitchingEquipment"))

(event Custom|Server_DisableControlRotation
  ;[0 0 0 1 30] Replicated_UseControlRotation
  (CallFunction|MCDisableControlRotation))

(event Custom|MC_DisableControlRotation
  ;[0 0 0 1 30] Replicated_UseControlRotation
  (Variables|/Script/Engine.CharacterMovementComponent|SetbUseControllerDesiredRotation (Variables|Character|GetCharacterMovement) false))

(event Custom|Server_EquipAnimLayer
  (params (AnimLayerComponent :type Actor%20Component%20Object%20Reference) (AnimLayer :type Anim%20Instance%20Class%20Reference))
  ;[0 0 0 1 30] EquipAnimLayer_Replication
  (CallFunction|MCEquipAnimLayer AnimLayerComponent AnimLayer))

(event Custom|Server_UseControlRotation
  ;[0 0 0 1 30] Replicated_UseControlRotation
  (CallFunction|MCUseControlRotation))

(event Custom|MC_UseControlRotation
  ;[0 0 0 1 30] Replicated_UseControlRotation
  (Variables|/Script/Engine.CharacterMovementComponent|SetbUseControllerDesiredRotation (Variables|Character|GetCharacterMovement) true))

(event Input|EnhancedActionEvents|EnhancedInputActionIA_MoveForward
  (params (ActionValue :type Float%20%28double-precision%29) (ElapsedSeconds :type Float%20%28double-precision%29) (TriggeredSeconds :type Float%20%28double-precision%29) (InputAction :type Input%20Action%20Object%20Reference :default "/Game/CombatContent/Characters/Player/PlayerInput/IA_MoveForward.IA_MoveForward"))
  ;[0 0 0 1 50] Movement
  (:Triggered
    (Pawn|Input|AddMovementInput (Math|Vector|GetForwardVector (Math|Rotator|MakeRotator 0.0 0.0 (.Yaw (Math|Rotator|BreakRotator (Pawn|GetControlRotation :!class /Script/Engine.Pawn))))) ActionValue false :!label _label))
  (:Started
    (goto _label))
  (:Ongoing
    (goto _label)))

(event Input|EnhancedActionEvents|EnhancedInputActionIA_MoveRight
  (params (ActionValue :type Float%20%28double-precision%29) (ElapsedSeconds :type Float%20%28double-precision%29) (TriggeredSeconds :type Float%20%28double-precision%29) (InputAction :type Input%20Action%20Object%20Reference :default "/Game/CombatContent/Characters/Player/PlayerInput/IA_MoveRight.IA_MoveRight"))
  ;[0 0 0 1 50] Movement
  (:Triggered
    (Utilities|IsGrounded :!label _label
      (:Grounded
        _)
      (:NotGrounded
        _))
    (Pawn|Input|AddMovementInput (Math|Vector|GetRightVector (Math|Rotator|MakeRotator 0.0 0.0 (.Yaw (Math|Rotator|BreakRotator (Pawn|GetControlRotation :!class /Script/Engine.Pawn))))) ActionValue false))
  (:Started
    (goto _label))
  (:Ongoing
    (goto _label)))

(event Input|EnhancedActionEvents|EnhancedInputActionIA_LookRight
  (params (ActionValue :type Float%20%28double-precision%29) (ElapsedSeconds :type Float%20%28double-precision%29) (TriggeredSeconds :type Float%20%28double-precision%29) (InputAction :type Input%20Action%20Object%20Reference :default "/Game/CombatContent/Characters/Player/PlayerInput/IA_LookRight.IA_LookRight"))
  ;[0 0 0 1 30] Camera_Turn and Look up
  (:Triggered
    (Pawn|Input|AddControllerYawInput ActionValue :!label _label))
  (:Started
    (goto _label)))

(event Input|EnhancedActionEvents|EnhancedInputActionIA_LookUp
  (params (ActionValue :type Float%20%28double-precision%29) (ElapsedSeconds :type Float%20%28double-precision%29) (TriggeredSeconds :type Float%20%28double-precision%29) (InputAction :type Input%20Action%20Object%20Reference :default "/Game/CombatContent/Characters/Player/PlayerInput/IA_LookUp.IA_LookUp"))
  ;[0 0 0 1 30] Camera_Turn and Look up
  (:Triggered
    (Pawn|Input|AddControllerPitchInput ActionValue :!label _label))
  (:Started
    (goto _label)))

(event EventBeginPlay
  ;[0 0 0] Register to GameplayFramework
  (Class|GameFrameworkComponentManager|AddReceiver (Subsystems|GetGameFrameworkComponentManager))
  (Variables|/Script/Engine.CharacterMovementComponent|SetMaxWalkSpeed (Variables|Character|GetCharacterMovement) (Variables|Default|GetWalkSpeed))
  (Variables|/Script/Engine.CharacterMovementComponent|SetMaxAcceleration (Variables|Character|GetCharacterMovement) (Variables|Default|GetMaxAcceleration))
  (Variables|/Script/Engine.CharacterMovementComponent|SetRotationRate (Variables|Character|GetCharacterMovement) (Variables|Default|GetDefailtRotationRate))
  (Variables|Default|SetCameraComponent (Variables|Camera|GetFollowCamera))
  (for _array_element (Class|Actor|GetComponentsbyInterface "/Game/CombatContent/Global_Components/WeaponLayerGlobals/BPI_LinkAnimLayers.BPI_LinkAnimLayers_C")
    (Utilities|Array|AddUnique (Variables|Character|AnimationLayerComponents|GetAnimLayerComponentsArray) _array_element))
  (Variables|Default|SetAnimLayerLength (- (Utilities|Array|Length (Variables|Character|AnimationLayerComponents|GetAnimLayerComponentsArray)) 1)))

(event EventTick
  (params (DeltaSeconds :type Float%20%28single-precision%29))
  (|CallParentFunction DeltaSeconds)
  (if (Class|GSCBlueprintFunctionLibrary|HasMatchingGameplayTag self "(TagName=\"Player.State.IsDashing\")")
    (CallFunction|SetCameraTargetLength 5e+02 DeltaSeconds)
    (else
      (CallFunction|SetCameraTargetLength (Variables|Default|GetDefaultTargetArmLength) DeltaSeconds)))
  (if (Class|GSCBlueprintFunctionLibrary|HasMatchingGameplayTag self "(TagName=\"Player.Loose.isLockON\")")
    (CallFunction|SetCameraLocationEvent "-300.000000,150.000000,100.000000" DeltaSeconds)
    (else
      (CallFunction|SetCameraLocationEvent (Variables|Default|GetDefaultSocketOffset) DeltaSeconds))))

(event EventRestarted
  ;[0 0 0] Character ClientSide Initialization
  (if (Pawn|IsLocallyControlled)
    (Utilities|IsValid (Variables|Character|UI|GetHUD)
      (:Is%20Not%20Valid
        (bind _asplayer_controller (Utilities|Casting|CastToPlayerController (Pawn|GetController)))
        (bind _returnvalue (UserInterface|CreateWidget "/Game/CombatContent/Characters/Player/PlayerUI/CombatWB_HUD.CombatWB_HUD_C" _asplayer_controller))
        (bind _output_get (Variables|Character|UI|SetHUD _returnvalue))
        (UserInterface|Viewport|AddtoViewport _output_get 0)))))

(event Input|KeyboardEvents|F
  (params (Key :type Key%20Structure :default "None"))
  ;[0 0 0] SwitchEquipment
  (:Pressed
    (CallFunction|ServerGetAnimLayerComponent)))

(event OnPreAttributeChange(GSCCore)
  (params (AttributeSet :type GSC%20Attribute%20Set%20Base%20Object%20Reference) (Attribute :type Gameplay%20Attribute%20Structure) (NewValue :type Float%20%28single-precision%29))
  (bind _gsccore (Variables|Default|GetGSCCore))
  ;[1 1 1] MaxChange
  (|SwitchGameplayAttribute Attribute
    (:MaxHealth
      (Class|GSCCoreComponent|AdjustAttributeforMaxChange _gsccore AttributeSet "(AttributeName=\"Health\",Attribute=/Script/CombatGASCompanion.CombatBaseAttributeSet:Health,AttributeOwner=/Script/CoreUObject.Class'\"/Script/CombatGASCompanion.CombatBaseAttributeSet\"')" "(AttributeName=\"MaxHealth\",Attribute=/Script/CombatGASCompanion.CombatBaseAttributeSet:MaxHealth,AttributeOwner=/Script/CoreUObject.Class'\"/Script/CombatGASCompanion.CombatBaseAttributeSet\"')" NewValue))
    (:MaxArmor
      (Class|GSCCoreComponent|AdjustAttributeforMaxChange _gsccore AttributeSet "(AttributeName=\"Armor\",Attribute=/Script/CombatGASCompanion.CombatBaseAttributeSet:Armor,AttributeOwner=/Script/CoreUObject.Class'\"/Script/CombatGASCompanion.CombatBaseAttributeSet\"')" "(AttributeName=\"MaxArmor\",Attribute=/Script/CombatGASCompanion.CombatBaseAttributeSet:MaxArmor,AttributeOwner=/Script/CoreUObject.Class'\"/Script/CombatGASCompanion.CombatBaseAttributeSet\"')" NewValue))))

(event OnPostGameplayEffectExecute(GSCCore)
  (params (Attribute :type Gameplay%20Attribute%20Structure) (SourceActor :type Actor%20Object%20Reference) (TargetActor :type Actor%20Object%20Reference) (SourceTags :type Gameplay%20Tag%20Container%20Structure%20%28by%20ref%29) (Payload :type GSC%20Gameplay%20Effect%20Execute%20Data%20Structure))
  ;[1 1 1] PostGameplayEffectExecution(Clamps)
  (|SwitchGameplayAttribute Attribute
    (:Health
      (ClampHelpers|ClampHealth "(AttributeName=\"Health\",Attribute=/Script/CombatGASCompanion.CombatBaseAttributeSet:Health,AttributeOwner=/Script/CoreUObject.Class'\"/Script/CombatGASCompanion.CombatBaseAttributeSet\"')"))
    (:Armor
      (ClampHelpers|ClampArmor "(AttributeName=\"Armor\",Attribute=/Script/CombatGASCompanion.CombatBaseAttributeSet:Armor,AttributeOwner=/Script/CoreUObject.Class'\"/Script/CombatGASCompanion.CombatBaseAttributeSet\"')"))))

(fn ConstructionScript)

(fn ClampHealth
  (params (Attribute :type Gameplay%20Attribute%20Structure))
  (bind _gsccore (Variables|Default|GetGSCCore))
  (Class|GSCCoreComponent|ClampAttributeValue _gsccore Attribute 0.0 (Class|GSCCoreComponent|GetAttributeValue _gsccore "(AttributeName=\"MaxHealth\",Attribute=/Script/CombatGASCompanion.CombatBaseAttributeSet:MaxHealth,AttributeOwner=/Script/CoreUObject.Class'\"/Script/CombatGASCompanion.CombatBaseAttributeSet\"')")))

(fn ClampArmor
  (params (Attribute :type Gameplay%20Attribute%20Structure))
  (bind _gsccore (Variables|Default|GetGSCCore))
  (Class|GSCCoreComponent|ClampAttributeValue _gsccore Attribute 0.0 (Class|GSCCoreComponent|GetAttributeValue _gsccore "(AttributeName=\"MaxArmor\",Attribute=/Script/CombatGASCompanion.CombatBaseAttributeSet:MaxArmor,AttributeOwner=/Script/CoreUObject.Class'\"/Script/CombatGASCompanion.CombatBaseAttributeSet\"')")))

(fn GetAnimLayerComponent
  (bind _self self)
  (if (>= (Variables|Default|GetCurrentAnimLayer) (Variables|Default|GetAnimLayerLength))
    (Variables|Default|SetCurrentAnimLayer 0)
    (else
      (Math|Integer|IncrementInt (Variables|Default|GetCurrentAnimLayer)
        (:%20%20
          _))))
  (bind _asbpc_base_anim_layer_component (Utilities|Casting|CastToBPC_BaseAnimLayerComponent (Utilities|Array|Get(acopy) (Variables|Character|AnimationLayerComponents|GetAnimLayerComponentsArray) (Variables|Default|GetCurrentAnimLayer))))
  (bind _output_get (Variables|Character|AnimationLayerComponents|SetAnimLayerComponent _asbpc_base_anim_layer_component))
  (Utilities|RemoveWeaponStateTagEffects)
  (GameplayEffects|ApplyGameplayEffectSpecToSelf (Ability|GetAbilitySystemComponent _self) (GameplayEffects|MakeOutgoingSpec :self (Ability|GetAbilitySystemComponent _self) :GameplayEffectClass (Variables|/Game/CombatContent/Global_Components/WeaponLayerGlobals/BPC_BaseAnimLayerComponent.BPC_BaseAnimLayerComponent_C|GetWeaponTagEffect _asbpc_base_anim_layer_component)))
  (return _output_get (Variables|/Game/CombatContent/Global_Components/WeaponLayerGlobals/BPC_BaseAnimLayerComponent.BPC_BaseAnimLayerComponent_C|GetAnimLayer _asbpc_base_anim_layer_component)))

(fn GetWalkSpeedandMaxWalkSpeed
  (return (Variables|Default|GetWalkSpeed) (Variables|Default|GetSprintSpeed) (Variables|Default|GetDefailtRotationRate)))

(fn GetBaseWeapon
  (for _array_element (Actor|GetAttachedActors true false)
    (bind _asbp_weapon_base (Utilities|Casting|CastToBP_WeaponBase _array_element))
    (return _asbp_weapon_base)))

(fn SetCameraLocationEvent
  (params (Socket%20Offset :type Vector) (DeltaTime :type Float%20%28single-precision%29))
  (Variables|/Script/Engine.SpringArmComponent|SetSocketOffset (Variables|Camera|GetCameraBoom) (Math|Interpolation|VInterpTo (Variables|/Script/Engine.SpringArmComponent|GetSocketOffset (Variables|Camera|GetCameraBoom)) Socket%20Offset DeltaTime 1.0)))

(fn SetCameraTargetLength
  (params (TargetArmLength :type Float%20%28double-precision%29) (DeltaTime :type Float%20%28double-precision%29))
  (Variables|/Script/Engine.SpringArmComponent|SetTargetArmLength (Variables|Camera|GetCameraBoom) (Math|Interpolation|FInterpTo (Variables|/Script/Engine.SpringArmComponent|GetTargetArmLength (Variables|Camera|GetCameraBoom)) TargetArmLength DeltaTime 1.0)))

(fn GetDefaultMaxAcceleration
  (return (Variables|Default|GetMaxAcceleration)))