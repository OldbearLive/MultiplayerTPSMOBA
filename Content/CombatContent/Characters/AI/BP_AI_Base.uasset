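; Base AI combat character built on the Gameplay Ability System, with an attribute-bound health bar widget.
; An aggro sphere collects overlapping base characters and sets the target, picking randomly when one re-enters.
; Incoming damage applies a SetByCaller gameplay effect, spawns randomly scaled damage numbers and sends hit-stop, which pauses animation and movement until a timer ends it.
; GSCCore callbacks clamp health and armor and adjust them when maximums change.
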(event OnComponentBeginOverlap(AggroCollision)
  (params (OverlappedComponent :type Primitive%20Component%20Object%20Reference) (OtherActor :type Actor%20Object%20Reference) (OtherComp :type Primitive%20Component%20Object%20Reference) (OtherBodyIndex :type Integer) (bFromSweep :type Boolean) (SweepResult :type Hit%20Result%20Structure%20%28by%20ref%29))
  (bind _targetactorsarray (Variables|Default|GetTargetActorsArray))
  (bind _targetactorsarray_2 (Variables|Default|GetTargetActorsArray))
  ;[0 0 0] AggroCollision TargetCalculation
  (bind _asbp_base_character (Utilities|Casting|CastToBP_BaseCharacter OtherActor))
  (if (Utilities|Array|ContainsItem _targetactorsarray _asbp_base_character)
    (Variables|Default|SetTargetActor (Utilities|Array|Get(acopy) _targetactorsarray_2 (Math|Random|RandomIntegerinRange 0 (- (Utilities|Array|Length _targetactorsarray_2) 1))))
    (else
      (bind _returnvalue (Utilities|Array|AddUnique _targetactorsarray _asbp_base_character))
      (Variables|Default|SetTargetActor (Utilities|Array|Get(acopy) (Variables|Default|GetTargetActorsArray) _returnvalue)))))

(event Custom|CheckTargets
  (bind _targetactorsarray (Variables|Default|GetTargetActorsArray))
  (bind _targetactorsarray_2 (Variables|Default|GetTargetActorsArray))
  ;[0 0 0] AggroCollision TargetCalculation
  (if (Utilities|Array|ContainsItem _targetactorsarray (stale OnComponentBeginOverlap(AggroCollision) _asbp_base_character))
    (Variables|Default|SetTargetActor (Utilities|Array|Get(acopy) _targetactorsarray_2 (Math|Random|RandomIntegerinRange 0 (- (Utilities|Array|Length _targetactorsarray_2) 1))))
    (else
      (bind _returnvalue (Utilities|Array|AddUnique _targetactorsarray (stale OnComponentBeginOverlap(AggroCollision) _asbp_base_character)))
      (Variables|Default|SetTargetActor (Utilities|Array|Get(acopy) (Variables|Default|GetTargetActorsArray) _returnvalue)))))

(event EventHandleInstantDamage
  (params (WeaponRawDamage :type Float%20%28double-precision%29) (DamageOwnerActor :type Actor%20Object%20Reference) (HitStopDuration :type Float%20%28double-precision%29) (HitWorldLocation :type Vector :default "0, 0, 0"))
  (bind _returnvalue (Math|Random|RandomFloatinRange 0.5 1.0))
  (bind _abilitysystemcomponent (Variables|Default|GetAbilitySystemComponent))
  ;[0 0 0] AI_ Handle Damage
  (bind _returnvalue_2 (Ability|GameplayEffect|AssignTagSetbyCallerMagnitude (GameplayEffects|MakeOutgoingSpec _abilitysystemcomponent "/Game/CombatContent/Global_Components/Global_Abilities/AbilityEffects/GE_InstantDamage.GE_InstantDamage_C" 0.0 (GameplayEffects|MakeEffectContext _abilitysystemcomponent)) "(TagName=\"Data.Damage.DamageMagnitude\")" WeaponRawDamage))
  (GameplayEffects|ApplyGameplayEffectSpecToSelf (Ability|GetAbilitySystemComponent self) _returnvalue_2)
  (bind _returnvalue_3 (AddComponent|AddWidgetComponent false (Math|Transform|MakeTransform (Math|Transform|InverseTransformLocation (Transformation|GetActorTransform) HitWorldLocation) "0, 0, 0" "0.100000,0.100000,0.100000")))
  (bind _aswb_damage_numbers (Utilities|Casting|CastToWB_DamageNumbers (UserInterface|GetWidget _returnvalue_3)))
  (Widget|Transform|SetRenderScale _aswb_damage_numbers (Math|Vector2D|MakeVector2D _returnvalue _returnvalue))
  (Default|UpdateDamageNumber _aswb_damage_numbers WeaponRawDamage)
  (Utilities|FlowControl|RetriggerableDelay 0.05)
  (Class|BPIDamageInterface|HandleHitstop(Message) self HitStopDuration DamageOwnerActor))

(event EventHandleHitstop
  (params (HitStopDuration :type Float%20%28double-precision%29) (DamageOwnerActor :type Actor%20Object%20Reference))
  ;[0 0 0] HandleHitStip
  (Variables|/Script/Engine.SkeletalMeshComponent|SetbPauseAnims (Variables|Character|GetMesh) true)
  (Components|Movement|StopMovementImmediately (Variables|Character|GetCharacterMovement))
  (Utilities|Time|SetTimerbyFunctionName 0 "EndHitStop" HitStopDuration))

(event EventRestarted)

(event EventBeginPlay
  (Utilities|Array|Clear (Variables|Default|GetTargetActorsArray))
  (Variables|Default|SetTargetActor 0)
  (bind _aswb_ai_health_bar (Utilities|Casting|CastToWB_AI_HealthBar (UserInterface|GetUserWidgetObject (Variables|Default|GetAIHealthArmor))))
  (Class|GSCUserWidget|InitializewithAbilitySystem _aswb_ai_health_bar (Variables|Default|GetAbilitySystemComponent)))

(event EventHandleCanAttackProbability
  (params (DamageDealer :type Actor%20Object%20Reference))
  (Ability|SendGameplayEventtoActor self "(TagName=\"Event.AI.CanAttack\")"))

(event OnPreAttributeChange(GSCCore)
  (params (AttributeSet :type GSC%20Attribute%20Set%20Base%20Object%20Reference) (Attribute :type Gameplay%20Attribute%20Structure) (NewValue :type Float%20%28single-precision%29))
  (bind _gsccore (Variables|Default|GetGSCCore))
  ;[0 0 0] MaxChange
  (|SwitchGameplayAttribute Attribute
    (:MaxHealth
      (Class|GSCCoreComponent|AdjustAttributeforMaxChange _gsccore AttributeSet "(AttributeName=\"Health\",Attribute=/Script/CombatGASCompanion.CombatBaseAttributeSet:Health,AttributeOwner=/Script/CoreUObject.Class'\"/Script/CombatGASCompanion.CombatBaseAttributeSet\"')" "(AttributeName=\"MaxHealth\",Attribute=/Script/CombatGASCompanion.CombatBaseAttributeSet:MaxHealth,AttributeOwner=/Script/CoreUObject.Class'\"/Script/CombatGASCompanion.CombatBaseAttributeSet\"')" NewValue))
    (:MaxArmor
      (Class|GSCCoreComponent|AdjustAttributeforMaxChange _gsccore AttributeSet "(AttributeName=\"Armor\",Attribute=/Script/CombatGASCompanion.CombatBaseAttributeSet:Armor,AttributeOwner=/Script/CoreUObject.Class'\"/Script/CombatGASCompanion.CombatBaseAttributeSet\"')" "(AttributeName=\"MaxArmor\",Attribute=/Script/CombatGASCompanion.CombatBaseAttributeSet:MaxArmor,AttributeOwner=/Script/CoreUObject.Class'\"/Script/CombatGASCompanion.CombatBaseAttributeSet\"')" NewValue))))

(event OnPostGameplayEffectExecute(GSCCore)
  (params (Attribute :type Gameplay%20Attribute%20Structure) (SourceActor :type Actor%20Object%20Reference) (TargetActor :type Actor%20Object%20Reference) (SourceTags :type Gameplay%20Tag%20Container%20Structure%20%28by%20ref%29) (Payload :type GSC%20Gameplay%20Effect%20Execute%20Data%20Structure))
  ;[0 0 0] PostGameplayEffectExecution(Clamps)
  (|SwitchGameplayAttribute Attribute
    (:Health
      (CallFunction|ClampHealth "(AttributeName=\"Health\",Attribute=/Script/CombatGASCompanion.CombatBaseAttributeSet:Health,AttributeOwner=/Script/CoreUObject.Class'\"/Script/CombatGASCompanion.CombatBaseAttributeSet\"')"))
    (:Armor
      (CallFunction|ClampArmor "(AttributeName=\"Armor\",Attribute=/Script/CombatGASCompanion.CombatBaseAttributeSet:Armor,AttributeOwner=/Script/CoreUObject.Class'\"/Script/CombatGASCompanion.CombatBaseAttributeSet\"')"))))

(fn ConstructionScript
  (Components|Sphere|SetSphereRadius (Variables|Default|GetAggroCollision) (Variables|Default|GetAggroSphereRadius) true))

(fn EndHitStop
  (Variables|/Script/Engine.SkeletalMeshComponent|SetbPauseAnims (Variables|Character|GetMesh) false)
  (Variables|Default|SetCustomTimeDilation 1.0))

(fn ClampHealth
  (params (Attribute :type Gameplay%20Attribute%20Structure))
  (bind _gsccore (Variables|Default|GetGSCCore))
  (Class|GSCCoreComponent|ClampAttributeValue _gsccore Attribute 0.0 (Class|GSCCoreComponent|GetAttributeValue _gsccore "(AttributeName=\"MaxHealth\",Attribute=/Script/CombatGASCompanion.CombatBaseAttributeSet:MaxHealth,AttributeOwner=/Script/CoreUObject.Class'\"/Script/CombatGASCompanion.CombatBaseAttributeSet\"')")))

(fn ClampArmor
  (params (Attribute :type Gameplay%20Attribute%20Structure))
  (bind _gsccore (Variables|Default|GetGSCCore))
  (Class|GSCCoreComponent|ClampAttributeValue _gsccore Attribute 0.0 (Class|GSCCoreComponent|GetAttributeValue _gsccore "(AttributeName=\"MaxArmor\",Attribute=/Script/CombatGASCompanion.CombatBaseAttributeSet:MaxArmor,AttributeOwner=/Script/CoreUObject.Class'\"/Script/CombatGASCompanion.CombatBaseAttributeSet\"')")))

(fn CanHandleAttack
  (params (Actor :type Actor%20Object%20Reference)))

(fn GetSkeletalMeshComponent
  (return 0))