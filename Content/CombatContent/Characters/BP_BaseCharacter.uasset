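; Base combat character that handles incoming damage, hit stop and target lock-on.
; Damage applies a SetByCaller GAS effect, notifies the attacker, spawns a randomly scaled damage-number widget, then requests server hit stop after a brief delay.
; Hit stop pauses mesh animation and zeroes acceleration until a timer restores them.
; Lock-on steers control rotation on Tick with clamped pitch, breaks beyond range, and sets orient-to-movement from the sword layer tag.
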(event Custom|SwitchingEquipment
  (Utilities|IsValid (Variables|Default|GetLock%20on%20Target)
    (:Is%20Valid
      (CallFunction|SwitchingEquipmentCheck))))

(event Custom|SwitchingEquipmentCheck
  (if (Class|GSCBlueprintFunctionLibrary|HasMatchingGameplayTag self "(TagName=\"Weapon.Layer.Sword\")")
    (Variables|/Script/Engine.CharacterMovementComponent|SetbOrientRotationToMovement (Variables|Character|GetCharacterMovement) true)
    (else
      (Variables|/Script/Engine.CharacterMovementComponent|SetbOrientRotationToMovement (Variables|Character|GetCharacterMovement) false))))

(event Custom|MC_HandleHitStop
  (params (Target :type Object%20Object%20Reference) (HitStopDuration :type Float%20%28double-precision%29)))

(event Custom|Server_HandleHitStop
  (params (Target :type Object%20Object%20Reference) (HitStopDuration :type Float%20%28double-precision%29))
  (Class|BPIDamageInterface|HandleHitstop(Message) Target HitStopDuration))

(event EventBeginPlay
  (Variables|Default|SetLock%20on%20Target 0))

(event EventOnLanded
  (params (Hit :type Hit%20Result%20Structure%20%28by%20ref%29))
  (Ability|SendGameplayEventtoActor self "(TagName=\"Player.Event.Landed\")"))

(event EventTick
  (params (DeltaSeconds :type Float%20%28single-precision%29))
  ;[1 1 1 1 100] LockOnEventTick
  (if (Utilities|IsValid (Variables|Default|GetLock%20on%20Target))
    (if (> (Transformation|GetDistanceTo (Variables|Default|GetLock%20on%20Target)) 2e+03)
      (Utilities|IsValid (Variables|Default|GetLock%20on%20Target)
        (:Is%20Valid
          (Variables|Default|SetLock%20on%20Target 0)
          (Ability|GameplayEffect|RemoveLooseGameplayTags self (GameplayTags|MakeGameplayTagContainerfromArray (Utilities|Array|MakeArray "(TagName=\"Player.Loose.isLockON\")")))
          (Class|BPIGetPlayerInfo|DiableLockON(Message) self)))
      (else
        (Pawn|SetControlRotation (Pawn|GetController) (Math|Rotator|MakeRotator (.Roll (Math|Rotator|BreakRotator (Pawn|GetControlRotation :!class /Script/Engine.Pawn))) (Math|Float|ClampAngle (.Pitch (Math|Rotator|BreakRotator (Math|Rotator|FindLookatRotation (Transformation|GetActorLocation) (Transformation|GetActorLocation (Variables|Default|GetLock%20on%20Target))))) -15.0 15.0) (.Yaw (Math|Rotator|BreakRotator (Math|Rotator|FindLookatRotation (Transformation|GetActorLocation) (Transformation|GetActorLocation (Variables|Default|GetLock%20on%20Target)))))))))))

(event EventHandleInstantDamage
  (params (WeaponRawDamage :type Float%20%28double-precision%29) (DamageOwnerActor :type Actor%20Object%20Reference) (HitStopDuration :type Float%20%28double-precision%29) (HitWorldLocation :type Vector :default "0, 0, 0"))
  (bind _returnvalue (Math|Random|RandomFloatinRange 0.25 0.5))
  (bind _self self)
  (bind _returnvalue_2 (Ability|GetAbilitySystemComponent _self))
  ;[1 1 1] HandleDamage
  (Ability|SendGameplayEventtoActor DamageOwnerActor "(TagName=\"Event.AI.Received.Hit\")")
  (bind _returnvalue_3 (Ability|GameplayEffect|AssignTagSetbyCallerMagnitude (GameplayEffects|MakeOutgoingSpec _returnvalue_2 "/Game/CombatContent/Global_Components/Global_Abilities/AbilityEffects/GE_InstantDamage.GE_InstantDamage_C" 0.0 (GameplayEffects|MakeEffectContext _returnvalue_2)) "(TagName=\"Data.Damage.DamageMagnitude\")" WeaponRawDamage))
  (GameplayEffects|ApplyGameplayEffectSpecToSelf (Ability|GetAbilitySystemComponent self) _returnvalue_3)
  (bind _returnvalue_4 (AddComponent|AddWidgetComponent false (Math|Transform|MakeTransform (Math|Transform|InverseTransformLocation (Transformation|GetActorTransform) HitWorldLocation) "0, 0, 0" "0.100000,0.100000,0.100000")))
  (bind _aswb_damage_numbers (Utilities|Casting|CastToWB_DamageNumbers (UserInterface|GetWidget _returnvalue_4)))
  (Widget|Transform|SetRenderScale _aswb_damage_numbers (Math|Vector2D|MakeVector2D _returnvalue _returnvalue))
  (Default|UpdateDamageNumber _aswb_damage_numbers WeaponRawDamage)
  (Utilities|FlowControl|RetriggerableDelay 0.05)
  (CallFunction|ServerHandleHitStop self HitStopDuration))

(event Collision|EventActorBeginOverlap
  (params (OtherActor :type Actor%20Object%20Reference)))

(event EventHandleLockON
  (params (LockOnTarget :type Actor%20Object%20Reference))
  (Utilities|IsValid LockOnTarget
    (:Is%20Valid
      (Variables|Default|SetLock%20on%20Target LockOnTarget)
      (Actor|Tick|SetActorTickEnabled self true)
      (if (Class|GSCBlueprintFunctionLibrary|HasMatchingGameplayTag self "(TagName=\"Weapon.Layer.Sword\")")
        (Variables|/Script/Engine.CharacterMovementComponent|SetbOrientRotationToMovement (Variables|Character|GetCharacterMovement) true)
        (else
          (Variables|/Script/Engine.CharacterMovementComponent|SetbOrientRotationToMovement (Variables|Character|GetCharacterMovement) false))))
    (:Is%20Not%20Valid
      (Actor|Tick|SetActorTickEnabled true)
      (Variables|Default|SetLock%20on%20Target 0)
      (Variables|/Script/Engine.CharacterMovementComponent|SetbOrientRotationToMovement (Variables|Character|GetCharacterMovement) true))))

(event EventDiableLockON
  (Actor|Tick|SetActorTickEnabled true)
  (Variables|Default|SetLock%20on%20Target 0)
  (Variables|/Script/Engine.CharacterMovementComponent|SetbOrientRotationToMovement (Variables|Character|GetCharacterMovement) true))

(event EventHandleHitstop
  (params (HitStopDuration :type Float%20%28double-precision%29) (DamageOwnerActor :type Actor%20Object%20Reference))
  (Variables|/Script/Engine.SkeletalMeshComponent|SetbPauseAnims (Variables|Character|GetMesh) true)
  (Variables|/Script/Engine.CharacterMovementComponent|SetMaxAcceleration (Variables|Character|GetCharacterMovement) 0.0)
  (Utilities|Time|SetTimerbyFunctionName 0 "StopHitStop" HitStopDuration))

(fn ConstructionScript)

(fn StopHitStop
  (Variables|/Script/Engine.SkeletalMeshComponent|SetbPauseAnims (Variables|Character|GetMesh) false)
  (Variables|/Script/Engine.CharacterMovementComponent|SetMaxAcceleration (Variables|Character|GetCharacterMovement) 2048.0))

(fn GetWalkSpeedandMaxWalkSpeed
  (return 0.0 0.0 "0, 0, 0"))

(fn GetBaseWeapon
  (return 0))

(fn GetSkeletalMeshComponent
  (return (Variables|Character|GetMesh)))